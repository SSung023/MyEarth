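; PlayerGameMode is a game mode that respawns the player and reloads a streamed level whenever the player character is destroyed.
; At BeginPlay it binds to the player character's OnDestroyed event.
; On destruction it unloads and reloads the named stream level, blocking on load, then spawns and possesses a new PlayerCharacter at a stored transform.
; It then calls Respawn to bind the new character, repeating the cycle.
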(event Custom|OnDestroyed_
  (params (DestroyedActor :type Actor%20Object%20Reference))
  (bind _levelname (Variables|Default|GetlevelName))
  (bind _returnvalue (Utilities|String|StringToName _levelname))
  (Game|UnloadStreamLevel(byName) _returnvalue false)
  (Game|LoadStreamLevel(byName) _returnvalue true true)
  (bind _returnvalue_2 (Game|SpawnActorfromClass "/Game/Blueprints/Character/feat_player/PlayerCharacter.PlayerCharacter_C" (Variables|Default|GetspawnTransform) "Undefined" 0 0))
  (Pawn|Possess (Game|GetPlayerController 0) _returnvalue_2)
  (CallFunction|Respawn))

(event Custom|Respawn
  (bind _asplayer_character (Utilities|Casting|CastToPlayerCharacter (Game|GetPlayerCharacter 0)))
  (Game|BindEventtoOnDestroyed _asplayer_character (delegate Custom|OnDestroyed_)))

(event EventBeginPlay
  (bind _asplayer_character (Utilities|Casting|CastToPlayerCharacter (Game|GetPlayerCharacter 0)))
  (Game|BindEventtoOnDestroyed _asplayer_character (delegate Custom|OnDestroyed_)))

(fn ConstructionScript)