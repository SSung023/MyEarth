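; Trigger volume that shows a tutorial UI while a player character stands inside it.
; Box overlap begin passes the configured TutorialImage and Shake to the PlayerCharacter's AttachTutorialUI, and overlap end calls DetachTutorialUI.
; The construction script sizes the box from the BoxExtent variable, so each placed instance can be fitted to its area.
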(event OnComponentBeginOverlap(Box)
  (params (OverlappedComponent :type Primitive%20Component%20Object%20Reference) (OtherActor :type Actor%20Object%20Reference) (OtherComp :type Primitive%20Component%20Object%20Reference) (OtherBodyIndex :type Integer) (bFromSweep :type Boolean) (SweepResult :type Hit%20Result%20Structure%20%28by%20ref%29))
  (bind _asplayer_character (Utilities|Casting|CastToPlayerCharacter OtherActor))
  (Default|AttachTutorialUI _asplayer_character (Variables|Option|GetTutorial%20Image) (Variables|Option|GetShake)))

(event OnComponentEndOverlap(Box)
  (params (OverlappedComponent :type Primitive%20Component%20Object%20Reference) (OtherActor :type Actor%20Object%20Reference) (OtherComp :type Primitive%20Component%20Object%20Reference) (OtherBodyIndex :type Integer))
  (bind _asplayer_character (Utilities|Casting|CastToPlayerCharacter OtherActor))
  (Default|DetachTutorialUI _asplayer_character))

(event EventBeginPlay)

(fn ConstructionScript
  (Components|Box|SetBoxExtent (Variables|Default|GetBox) (Variables|Option|GetBox%20Extent) true))