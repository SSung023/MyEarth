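; Trigger actor for a one-time aurora cutscene with the cormorant NPC, fired when the player overlaps it.
; Blends the view to a camera and auto-walks the player to a destination, then starts a delayed NPC chat while a timeline drives the weather manager's aurora intensity.
; EndChat blends the view back to the player and clears their chat-ready flag.
; The walk-speed override in MovePlayerTo is disconnected.
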(event OnComponentBeginOverlap(eventTrigger)
  (params (OverlappedComponent :type Primitive%20Component%20Object%20Reference) (OtherActor :type Actor%20Object%20Reference) (OtherComp :type Primitive%20Component%20Object%20Reference) (OtherBodyIndex :type Integer) (bFromSweep :type Boolean) (SweepResult :type Hit%20Result%20Structure%20%28by%20ref%29))
  (if (Actor|ActorHasTag OtherActor "Player")
    (CallFunction|AuroraEvent)))

(event Custom|endChat
  (bind _playerobj (Variables|Default|GetplayerObj))
  ;[1 1 1] Aurora Event
  (Game|Player|SetViewTargetwithBlend (Game|GetPlayerController 0) _playerobj 1.0 "VTBlend_Cubic" 0.0 false)
  (Variables|/Game/Blueprints/Character/feat_player/PlayerCharacter.PlayerCharacter_C|SetisReadyToChat _playerobj false))

(event Custom|turnAuroraCamera
  ;[1 1 1] Aurora Event
  (Game|Player|SetViewTargetwithBlend (Game|GetPlayerController 0) (Variables|Default|Getcamera) 1.0 "VTBlend_Linear" 0.0 false))

(event Custom|auroraEvent
  ;[1 1 1] Aurora Event
  (if (not (Variables|Default|GetisAuroraFinished))
    (Variables|Default|SetisAuroraFinished true)
    (Game|Player|SetViewTargetwithBlend (Game|GetPlayerController 0) (Variables|Default|Getcamera) 1.0 "VTBlend_Linear" 0.0 false)
    (CallFunction|MovePlayerto (Transformation|GetActorLocation (Variables|Default|Getdestination)) 1e+03)))

(event Custom|movePlayerTo
  (params (destination :type Vector) (speed :type Float%20%28single-precision%29))
  ;[1 1 1] Aurora Event
  (AI|Navigation|SimpleMovetoLocation (Game|GetPlayerController 0) destination)
  (CallFunction|StartChat 1.5)
  (CallFunction|PlayAurora))

(event Custom|playAurora
  (bind _weathermanager (Variables|Default|GetweatherManager))
  ;[1 1 1] Aurora Event
  (bind _intensity (Timeline|auroraIntensity PlayFromStart)
    (:Update
      (Variables|/Game/Blueprints/Weather/BP_WeatherManager.BP_WeatherManager_C|SetNext%20Aurora%20Intensity _weathermanager _intensity)
      (Default|TranslateAuroraIntensity _weathermanager))))

(event Custom|startChat
  (params (delay :type Float%20%28single-precision%29))
  (bind _npcobj (Variables|Default|GetnpcObj))
  ;[1 1 1] Aurora Event
  (Utilities|FlowControl|Delay delay)
  (Default|SetChatInfo _npcobj)
  (Variables|/Game/Blueprints/Character/feat_npc/BP_Cormorant.BP_Cormorant_C|SetisAurora _npcobj true)
  (Default|DeactivateParticle _npcobj 0.0)
  (Default|StartChat (Variables|Default|GetplayerObj) true))

(event EventBeginPlay
  (bind _asplayer_character (Utilities|Casting|CastToPlayerCharacter (Game|GetPlayerCharacter 0))
    (:then
      (Variables|Default|SetplayerObj _asplayer_character))
    (:CastFailed
      _))
  (bind _returnvalue (Actor|GetActorOfClass "/Game/Blueprints/Weather/BP_WeatherManager.BP_WeatherManager_C"))
  (Variables|Default|SetweatherManager _returnvalue)
  (bind _returnvalue_2 (Actor|GetActorOfClass "/Game/Blueprints/Character/feat_npc/BP_Cormorant.BP_Cormorant_C"))
  (Variables|Default|SetnpcObj _returnvalue_2))

(fn ConstructionScript)