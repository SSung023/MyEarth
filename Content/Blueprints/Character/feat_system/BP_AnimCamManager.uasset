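; BP_AnimCamManager stages an aurora camera moment when the player enters its trigger.
; Overlap by a "Player"-tagged actor blends the first player controller's view to its Camera, with no switch back in this graph.
; The same event passes NextAuroraIntensity to the level's BP_WeatherManager and calls TranslateAuroraIntensity.
; On BeginPlay it also sets a fixed time of day through the weather manager's UDS sky reference.
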(event OnComponentBeginOverlap(eventTrigger)
  (params (OverlappedComponent :type Primitive%20Component%20Object%20Reference) (OtherActor :type Actor%20Object%20Reference) (OtherComp :type Primitive%20Component%20Object%20Reference) (OtherBodyIndex :type Integer) (bFromSweep :type Boolean) (SweepResult :type Hit%20Result%20Structure%20%28by%20ref%29))
  (if (Actor|ActorHasTag OtherActor "Player")
    (CallFunction|AuroraEvent)))

(event Custom|auroraEvent
  (Game|Player|SetViewTargetwithBlend (Game|GetPlayerController 0) (Variables|Default|Getcamera) 1.0 "VTBlend_Linear" 0.0 false)
  (bind _returnvalue (Actor|GetActorOfClass "/Game/Blueprints/Weather/BP_WeatherManager.BP_WeatherManager_C"))
  (Variables|Default|SetweatherManager _returnvalue)
  (Variables|/Game/Blueprints/Weather/BP_WeatherManager.BP_WeatherManager_C|SetNext%20Aurora%20Intensity _returnvalue (Variables|Default|GetNext%20Aurora%20Intensity))
  (Default|TranslateAuroraIntensity _returnvalue))

(event EventBeginPlay
  (bind _returnvalue (Actor|GetActorOfClass "/Game/Blueprints/Weather/BP_WeatherManager.BP_WeatherManager_C"))
  (Variables|Default|SetweatherManager _returnvalue)
  (Variables|/Game/UltraDynamicSky/Blueprints/Ultra_Dynamic_Sky.Ultra_Dynamic_Sky_C|SetTime%20of%20Day (Variables|/Game/Blueprints/Weather/BP_WeatherManager.BP_WeatherManager_C|GetUDS (Variables|Default|GetweatherManager)) 2e+03))

(fn ConstructionScript)