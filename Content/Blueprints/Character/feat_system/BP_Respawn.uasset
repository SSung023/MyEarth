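; Respawn checkpoint that manages level streaming and records where the player respawns.
; When a Player-tagged actor overlaps SaveTrigger, it loads and shows the next maps with blocking loads, then unloads the listed old maps, all chosen by enum names.
; It then stores a spawn transform, raised above the checkpoint and yawed half a turn, plus the respawn map name on PlayerGameMode.
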(event OnComponentBeginOverlap(saveTrigger)
  (params (OverlappedComponent :type Primitive%20Component%20Object%20Reference) (OtherActor :type Actor%20Object%20Reference) (OtherComp :type Primitive%20Component%20Object%20Reference) (OtherBodyIndex :type Integer) (bFromSweep :type Boolean) (SweepResult :type Hit%20Result%20Structure%20%28by%20ref%29))
  (bind _returnvalue (Transformation|GetActorTransform))
  (bind (_location _rotation) (Math|Transform|BreakTransform _returnvalue))
  (if (Actor|ActorHasTag OtherActor "Player")
    (for _array_element (Variables|LevelStreaming|GetNextMapName)
      (Game|LoadStreamLevel(byName) (Utilities|String|StringToName (Utilities|String|EnumtoString _array_element)) true true))
    (for _array_element_2 (Variables|LevelStreaming|GetunloadMapNames)
      (Game|UnloadStreamLevel(byName) (Utilities|String|StringToName (Utilities|String|EnumtoString _array_element_2)) false))
    (bind _asplayer_game_mode (Utilities|Casting|CastToPlayerGameMode (Game|GetGameMode)))
    (Variables|/Game/Blueprints/Character/feat_system/PlayerGameMode.PlayerGameMode_C|SetspawnTransform _asplayer_game_mode (Math|Transform|MakeTransform (+ _location "0, 0,200.000000") (Math|Rotator|MakeRotator (.roll _rotation) (.pitch _rotation) (+ (.yaw _rotation) 1.8e+02))))
    (Variables|/Game/Blueprints/Character/feat_system/PlayerGameMode.PlayerGameMode_C|SetlevelName _asplayer_game_mode (Utilities|String|EnumtoString (Variables|Respawn|GetrespawnMapName)))))

(fn ConstructionScript)