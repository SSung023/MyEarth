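; BP_Particle is an actor in the character head VFX system that spawns a configurable Niagara effect at its own location.
; FlashParticle spawns the effect once after a RateParticle delay, while NpcHeadUpParticle spawns it immediately and stores the component in HeadUpParticle.
; NpcDeactivateParticle, Tick and the construction script are empty, and a copy of the delayed spawn chain is left unconnected.
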(event Custom|FlashParticle
  (Utilities|FlowControl|Delay (Variables|Default|GetRate_Particle))
  (Niagara|SpawnSystematLocation (Variables|Default|GetParticle) (Transformation|GetActorLocation)))

(event Custom|NpcHeadUpParticle
  (bind _returnvalue (Niagara|SpawnSystematLocation (Variables|Default|GetParticle) (Transformation|GetActorLocation)))
  (Variables|Default|SetheadUpParticle _returnvalue))

(event Custom|NpcDeactivateParticle)

(event EventTick
  (params (DeltaSeconds :type Float%20%28single-precision%29)))

(fn ConstructionScript)