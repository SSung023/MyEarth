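; Killer whale actor that launches the player penguin onto a designated destination glacier.
; While idle, it circles a center point on Tick by moving along the tangent of its radius.
; On detection, timelines turn it toward the player and hop it to a waiting position, then enable input.
; Climb makes the player jump and triggers a launch montage, then timelines rotate and arc the player to the glacier.
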(event OnComponentBeginOverlap(DetectArea)
  (params (OverlappedComponent :type Primitive%20Component%20Object%20Reference) (OtherActor :type Actor%20Object%20Reference) (OtherComp :type Primitive%20Component%20Object%20Reference) (OtherBodyIndex :type Integer) (bFromSweep :type Boolean) (SweepResult :type Hit%20Result%20Structure%20%28by%20ref%29))
  (bind _asplayer_character (Utilities|Casting|CastToPlayerCharacter OtherActor))
  (Utilities|Casting|CastToCapsuleComponent OtherComp)
  (Variables|Default|SetPlayerCharacter _asplayer_character)
  (Utilities|FlowControl|Delay 0.2)
  (Variables|Default|SetisPlayerDetected (not (Variables|Default|GetisPlayerDetected)))
  (CallFunction|DetectPlayer))

(event OnComponentEndOverlap(DetectArea)
  (params (OverlappedComponent :type Primitive%20Component%20Object%20Reference) (OtherActor :type Actor%20Object%20Reference) (OtherComp :type Primitive%20Component%20Object%20Reference) (OtherBodyIndex :type Integer))
  (Utilities|Casting|CastToPlayerCharacter OtherActor)
  (Utilities|Casting|CastToCapsuleComponent OtherComp)
  (Utilities|FlowControl|Delay 0.2)
  (Variables|Default|SetisPlayerDetected (not (Variables|Default|GetisPlayerDetected)))
  (Animation|Montage|MontageStop (Variables|Default|GetAnimInstance) 0.3 "/Game/Resources/character/killerWhale/Montages/MT_KillerWhale_Detect.MT_KillerWhale_Detect"))

(event OnComponentBeginOverlap(MovableArea)
  (params (OverlappedComponent :type Primitive%20Component%20Object%20Reference) (OtherActor :type Actor%20Object%20Reference) (OtherComp :type Primitive%20Component%20Object%20Reference) (OtherBodyIndex :type Integer) (bFromSweep :type Boolean) (SweepResult :type Hit%20Result%20Structure%20%28by%20ref%29))
  (bind _asplayer_character (Utilities|Casting|CastToPlayerCharacter OtherActor))
  (Variables|Default|SetPlayerCharacter _asplayer_character))

(event Custom|Launch
  (bind _landingpos (Variables|Default|GetLandingPos))
  (bind _outputvector (Utilities|GETXYVECTOR _landingpos))
  ;[1 1 1] Launch Penguin
  (Utilities|FlowControl|DoOnce false :!label _label
    (:Completed
      (Transformation|SetRelativeRotation (Variables|Default|GetKillerWhale) (Math|Rotator|MakeRotator 0.0 0.0 (Variables|Default|GetWaitingRotator)) false false)
      (Variables|Default|SetCurYawRotation (.yaw (Transformation|GetActorRotation (Variables|Default|GetPlayerCharacter))))
      (Input|DisableInput (Variables|Default|GetPlayerCharacter) 0)
      (Animation|Montage|PlayMontage (Variables|Default|GetKillerWhale) "/Game/Resources/character/killerWhale/Montages/MT_KillerWhale_Launch.MT_KillerWhale_Launch" 1.0 0.0 "Default"
        (:then
          (Utilities|FlowControl|Delay (Variables|Default|GetLaunchDelay))
          (bind _output_get (Variables|Default|SetLaunchPos (Transformation|GetActorLocation (Variables|Default|GetPlayerCharacter))))
          (Variables|Default|SetXYdistance (Math|Vector|Distance(Vector) (Utilities|GETXYVECTOR _output_get) _outputvector))
          (Variables|Default|SetZdistance (Math|Vector|Distance(Vector) (Utilities|GETZVECTOR _output_get) (Utilities|GETZVECTOR _landingpos)))
          (bind _alpha (Timeline|Rotation PlayFromStart)
            (:Update
              (Transformation|SetActorRotation (Variables|Default|GetPlayerCharacter) (Math|Rotator|MakeRotator 0.0 0.0 (Math|Interpolation|Ease "EaseOut" _alpha (Variables|Default|GetCurYawRotation) (.yaw (Math|Rotator|FindLookatRotation (Utilities|GETXYVECTOR _output_get) _outputvector)) 2.0))))
            (:Finished
              (Variables|Default|SetDirectionVec (Transformation|GetActorForwardVector (Variables|Default|GetPlayerCharacter)))
              (bind (_direction _up _front) (Timeline|타임라인_0 PlayFromStart)
                (:Update
                  (Transformation|SetActorLocation (Variables|Default|GetPlayerCharacter) (+ (* "0, 0,1.000000" (* _up (Variables|Default|GetZdistance))) (+ (Variables|Default|GetLaunchPos) (* (Variables|Default|GetDirectionVec) (* _front (Variables|Default|GetXYdistance) 1.0)))) false false))
                (:Finished
                  (Input|EnableInput (Variables|Default|GetPlayerCharacter) 0)
                  (Input|DisableInput 0)
                  (Variables|Default|SetPlayerCharacter 0)
                  (Variables|Default|SetisPlayerJump false)
                  (Variables|Default|SetjumpCnt 0.0)
                  (goto _label Reset))))))))))

(event Custom|DetectPlayer
  (bind _killerwhale (Variables|Default|GetKillerWhale))
  (Variables|/Game/Blueprints/Character/feat_player/PlayerCharacter.PlayerCharacter_C|SetisKillerWhaleFront (Variables|Default|GetPlayerCharacter) true)
  (Animation|Montage|MontagePlay (Variables|Default|GetAnimInstance) "/Game/Resources/character/killerWhale/Montages/MT_KillerWhale_Detect.MT_KillerWhale_Detect" 1.0 "MontageLength" 0.0 true)
  (Variables|Default|SetCurYawRotation (.yaw (Transformation|GetWorldRotation _killerwhale)))
  (Variables|Default|SetFromPos (Transformation|GetWorldLocation _killerwhale))
  (Variables|Default|SetToPos (Transformation|GetActorLocation (Variables|Default|GetPlayerCharacter)))
  (if (Variables|Default|GetisPlayerDetected)
    (bind _alpha (Timeline|타임라인_1 PlayFromStart) ; 플레이어 바라보기
      (:Update
        (Transformation|SetWorldRotation (Variables|Default|GetKillerWhale) (Math|Rotator|MakeRotator 0.0 0.0 (Math|Interpolation|Ease "EaseOut" _alpha (Variables|Default|GetCurYawRotation) (.yaw (Math|Rotator|FindLookatRotation (Utilities|GETXYVECTOR (Variables|Default|GetFromPos)) (Utilities|GETXYVECTOR (Variables|Default|GetToPos)))) 2.0)) false false))
      (:Finished
        (Variables|Default|SetFromPos (Variables|/Script/Engine.SceneComponent|GetRelativeLocation (Variables|Default|GetKillerWhale)))
        (bind _output_get (Variables|Default|SetToPos (Variables|Default|GetWaitingPos)))
        (Variables|Default|SetDirectionVec (Math|Vector|GetUnitDirection(Vector) (Utilities|GETXYVECTOR (Variables|Default|GetFromPos)) (Utilities|GETXYVECTOR (Variables|Default|GetToPos))))
        (Variables|Default|SetZdistance (Math|Vector|Distance(Vector) (Utilities|GETZVECTOR _output_get) (Utilities|GETZVECTOR (Variables|Default|GetFromPos))))
        (Variables|Default|SetXYdistance (Math|Vector|Distance(Vector) (Utilities|GETXYVECTOR _output_get) (Utilities|GETXYVECTOR (Variables|Default|GetFromPos))))
        (if (Variables|Default|GetisPlayerDetected)
          (bind (_direction _up _front _alpha_2) (Timeline|타임라인_2 PlayFromStart) ; 점프
            (:Update
              (Transformation|SetRelativeLocationAndRotation (Variables|Default|GetKillerWhale) (+ (* "0, 0,5.000000" (* _up -3e+01)) (+ (Variables|Default|GetFromPos) (* (Variables|Default|GetDirectionVec) (* _front (Variables|Default|GetXYdistance) 1.0)))) (Math|Rotator|MakeRotator 0.0 0.0 (Math|Interpolation|Ease "EaseOut" _alpha_2 (Variables|Default|GetCurYawRotation) (Variables|Default|GetWaitingRotator) 2.0)) false false))
            (:Finished
              (Input|EnableInput (Game|GetPlayerController 0))))
          (else
            (Timeline|타임라인_2 Stop)))))
    (else
      (Timeline|타임라인_1 Stop))))

(event Custom|Idle
  (params (deltaTime :type Float%20%28single-precision%29))
  (bind _rotatedirectionvec (Variables|Default|GetRotateDirectionVec))
  ;[1 1 1] Idle
  (Transformation|SetWorldLocationAndRotation (Variables|Default|GetKillerWhale) (+ (Transformation|GetWorldLocation (Variables|Default|GetKillerWhale)) (* _rotatedirectionvec (* deltaTime (Variables|Default|GetRotateSpeed)))) (Math|Conversions|RotationFromXVector _rotatedirectionvec) false false))

(event EventBeginPlay
  (Utilities|SETLANDINGPOS
    (:out
      (Utilities|SETCENTER
        (:out
          (Utilities|FlowControl|Sequence
            (:then_0
              (Collision|SetCollisionEnabled (Variables|Default|GetTail) "NoCollision"))
            (:then_1
              (Collision|SetCollisionEnabled (Variables|Default|GetMovableArea) "NoCollision"))
            (:then_2
              (Variables|Default|SetAnimInstance (Components|SkeletalMesh|GetAnimInstance (Variables|Default|GetKillerWhale))))))))))

(event EventTick
  (params (DeltaSeconds :type Float%20%28single-precision%29))
  (if (not (Variables|Default|GetisPlayerDetected))
    (if (not (Variables|Default|GetisPlayerJump))
      (Utilities|GETROTATEVECTOR
        (:output
          (CallFunction|Idle DeltaSeconds))))))

(event Input|ActionEvents|InputActionClimb
  (params (Key :type Key%20Structure :default "None"))
  (bind _playercharacter (Variables|Default|GetPlayerCharacter))
  (:Pressed
    (Variables|Default|SetisPlayerJump true)
    (if (<= (Variables|Default|GetjumpCnt) 0.0)
      (Character|Jump _playercharacter)
      (Variables|Default|SetjumpCnt (+ (Variables|Default|GetjumpCnt) 1.0))
      (CallFunction|Launch)))
  (:Released
    (Character|StopJumping _playercharacter)))

(fn ConstructionScript
  (bind _killerwhale (Variables|Default|GetKillerWhale))
  (bind _relativelocation (Variables|/Script/Engine.SceneComponent|GetRelativeLocation _killerwhale))
  (Variables|Default|SetWaitingRotator -1.8e+02)
  (Variables|Default|SetWaitingPos (Math|Vector|MakeVector (+ (.x _relativelocation) 1e+02) (.y _relativelocation) (.z _relativelocation))))

(fn SetCenter
  (bind _center (Variables|Default|GetCenter))
  (Transformation|SetRelativeLocation _center (+ (* "1.000000, 0,0.000000" (Variables|Default|GetRotateRadius)) (.location (Transformation|GetRelativeTransform (Variables|Default|GetKillerWhale)))) false false)
  (Variables|Default|SetRotateCenterPos (Transformation|GetWorldLocation _center))
  (return))