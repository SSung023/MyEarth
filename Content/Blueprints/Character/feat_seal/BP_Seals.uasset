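; Seal actor, sitting or lying, that plays a warning montage while the player is near and can be moved, turned or dropped.
; MoveSeal slides it by timeline, then a downward trace keeps it in place, drops it by whole cells, or sinks and destroys it in water or void.
; SealTurn eases mesh yaw using the player's position and facing.
; Optional socket-attached snow meshes are removed when it moves or falls.
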(event OnComponentBeginOverlap(inaccessibleCollision)
  (params (OverlappedComponent :type Primitive%20Component%20Object%20Reference) (OtherActor :type Actor%20Object%20Reference) (OtherComp :type Primitive%20Component%20Object%20Reference) (OtherBodyIndex :type Integer) (bFromSweep :type Boolean) (SweepResult :type Hit%20Result%20Structure%20%28by%20ref%29))
  (bind _skeletalmesh (Variables|Default|GetSkeletalMesh))
  ;[1 1 1] when player nearby
  (bind _asplayer_character (Utilities|Casting|CastToPlayerCharacter OtherActor))
  (Variables|Default|SetplayerCharacter _asplayer_character)
  (Variables|Default|SetisPlayerNear true)
  (if (Variables|Default|GetisLyingSeal)
    (Animation|Montage|PlayMontage _skeletalmesh "/Game/Resources/character/Seal/montage/MT_seal_lying_Warning_edited.MT_seal_lying_Warning_edited" 1.0 0.0 "Default")
    (else
      (Animation|Montage|PlayMontage _skeletalmesh "/Game/Resources/character/Seal/montage/MT_seal_sit_Warning.MT_seal_sit_Warning" 1.0 0.0 "Default"))))

(event OnComponentEndOverlap(inaccessibleCollision)
  (params (OverlappedComponent :type Primitive%20Component%20Object%20Reference) (OtherActor :type Actor%20Object%20Reference) (OtherComp :type Primitive%20Component%20Object%20Reference) (OtherBodyIndex :type Integer))
  (bind _sealaniminstance (Variables|Default|GetsealAnimInstance))
  ;[1 1 1] when player nearby
  (Utilities|Casting|CastToPlayerCharacter OtherActor)
  (Variables|Default|SetisPlayerNear false)
  (if (Variables|Default|GetisLyingSeal)
    (Animation|Montage|MontageStop _sealaniminstance 0.0 "/Game/Resources/character/Seal/montage/MT_seal_lying_Warning_edited.MT_seal_lying_Warning_edited")
    (else
      (Animation|Montage|MontageStop _sealaniminstance 0.0 "/Game/Resources/character/Seal/montage/MT_seal_sit_Warning.MT_seal_sit_Warning"))))

(event Custom|MoveSeal
  (params (directionVec :type Vector))
  ;[1 1 1] moving mechanism
  (Utilities|FlowControl|DoOnce false :!label _label
    (:Completed
      (CallFunction|RemoveSnow)
      (bind _output_get (Variables|Default|SetdirectionVec directionVec))
      (bind _newpos (Timeline|updateSealPos PlayFromStart)
        (:Update
          (Transformation|SetActorLocation (+ (* _output_get _newpos) (Variables|Default|GetcurSealPos)) false false))
        (:Finished
          (Variables|Default|SetcurSealPos (Transformation|GetActorLocation))
          (bind _disttofloor (CallFunction|GetDistancetoFloor))
          (if (== _disttofloor 0) ; 0인 경우 바닥이 있음
            (goto _label Reset)
            (else
              (CallFunction|PlayAnimwhenFall _disttofloor)
              (goto _label Reset))))))))

(event Custom|FallingSeal
  (params (distToFloor :type Integer))
  (bind _skeletalmesh (Variables|Default|GetSkeletalMesh))
  ;[1 1 1] seal falling mechanism
  (CallFunction|RemoveSnow)
  (Utilities|FlowControl|Delay 0.2)
  (bind _newheight (CallFunction|ConvertFloorHeight distToFloor))
  (bind _velocity (Timeline|SealFalling PlayFromStart)
    (:Update
      (Transformation|SetActorLocation (+ (* _velocity _newheight) (Variables|Default|GetcurSealPos)) false false))
    (:Finished
      (Variables|Default|SetcurSealPos (Transformation|GetActorLocation))
      (if (Variables|Default|GetisLyingSeal)
        (Animation|Montage|PlayMontage _skeletalmesh "/Game/Resources/character/Seal/montage/MT_seal_lying_fallToGlacier_edited.MT_seal_lying_fallToGlacier_edited" 1.2 0.0 "Falling")
        (else
          (Animation|Montage|PlayMontage _skeletalmesh "/Game/Resources/character/Seal/montage/MT_seal_sit_fallToGlacier.MT_seal_sit_fallToGlacier" 1.0 0.0 "Falling"))))))

(event Custom|snowySeal
  (CallFunction|PutSnowMesh))

(event Custom|SealTurn
  (bind _returnvalue (Transformation|GetActorLocation))
  (bind _playercharacter (Variables|Default|GetPlayerCharacter))
  (bind _skeletalmesh (Variables|Default|GetSkeletalMesh))
  (bind (_x _y) (Math|Vector|BreakVector _returnvalue))
  (bind _returnvalue_2 (Transformation|GetActorLocation _playercharacter))
  (bind (_x_2 _y_2) (Math|Vector|BreakVector _returnvalue_2))
  ;[1 1 1] rotate seal
  (bind _alpha (Timeline|rotateSeal PlayFromStart)
    (:Update
      (Transformation|SetWorldRotation _skeletalmesh (Math|Rotator|MakeRotator 0.0 0.0 (Math|Interpolation|Ease "EaseOut" _alpha (.yaw (Math|Rotator|FindLookatRotation (Math|Vector|MakeVector _x _y 0.0) (Math|Vector|MakeVector _x_2 _y_2 0.0))) (.yaw (Transformation|GetActorRotation _playercharacter)) 2.0)) false false)
      (Variables|Default|SetcurZRotation (Math|Interpolation|Ease "EaseOut" _alpha (.yaw (Math|Rotator|FindLookatRotation (Math|Vector|MakeVector _x _y 0.0) (Math|Vector|MakeVector _x_2 _y_2 0.0))) (.yaw (Transformation|GetActorRotation _playercharacter)) 2.0)))
    (:Finished
      (Transformation|SetWorldRotation _skeletalmesh (Math|Rotator|MakeRotator 0.0 0.0 (Variables|Default|GetcurZRotation)) false false))))

(event Custom|FallToWater
  ;[1 1 1] seal fall to water
  (CallFunction|RemoveSnow)
  (Animation|Montage|PlayMontage (Variables|Default|GetSkeletalMesh) "/Game/Resources/character/Seal/montage/MT_seal_fallToWater.MT_seal_fallToWater" 1.0 0.0 "Default"
    (:then
      (bind _drownamt (Timeline|FallingToSea PlayFromStart)
        (:Update
          (Transformation|SetActorLocation (+ _drownamt (Variables|Default|GetcurSealPos)) false false))
        (:Finished
          (Actor|SetLifeSpan 0.5))))))

(event Custom|removeSnow
  (bind _nosesnowmesh (Variables|Default|GetNoseSnowMesh))
  (bind _backsnowmesh (Variables|Default|GetBackSnowMesh))
  (bind _headsnowmesh (Variables|Default|GetHeadSnowMesh))
  (Utilities|FlowControl|Sequence
    (:then_0
      (Utilities|IsValid _nosesnowmesh
        (:Is%20Valid
          (Components|DestroyComponent _nosesnowmesh))))
    (:then_1
      (Utilities|IsValid _backsnowmesh
        (:Is%20Valid
          (Components|DestroyComponent _backsnowmesh))))
    (:then_2
      (Utilities|IsValid _headsnowmesh
        (:Is%20Valid
          (Components|DestroyComponent _headsnowmesh))))))

(event EventBeginPlay
  (Variables|Default|SetsealAnimInstance (Components|SkeletalMesh|GetAnimInstance (Variables|Default|GetSkeletalMesh))))

(fn ConstructionScript
  (Variables|Default|SetcurSealPos (Transformation|GetActorLocation)))

(fn GetDistancetoFloor
  (bind _returnvalue (Transformation|GetActorLocation))
  (bind _directionvec (Variables|Default|GetdirectionVec))
  (bind _returnvalue_2 (+ _returnvalue _directionvec))
  (bind _outhit (Collision|LineTraceByChannel _returnvalue_2 (+ _returnvalue_2 "0, 0,-500.000000") "TraceTypeQuery1" false 0 "ForDuration" true "(R=0.060760,G=0.000000,B=1.000000,A=1.000000)" "(R=0.868007,G=0.000000,B=1.000000,A=1.000000)" 2.0))
  (if (Utilities|IsValid (.HitActor (Collision|BreakHitResult _outhit)))
    (Utilities|Casting|CastToBP_water (.HitActor (Collision|BreakHitResult _outhit))
      (:then
        (return -1) ; 바닥이 없는 경우
      )
      (:CastFailed
        (if (!= (Math|Float|Truncate (/ (.Distance (Collision|BreakHitResult _outhit)) 1e+02)) 0)
          (return (Math|Float|Truncate (/ (.Distance (Collision|BreakHitResult _outhit)) 1e+02))) ; 바다표범이 n칸 떨어져야하는 경우
          (else
            (return 0) ; 바닥이 있는 경우
          ))))
    (else
      (return -1) ; 바닥이 없는 경우
    )))

(fn ConvertFloorHeight
  (params (distToFloor :type Integer))
  (if (== distToFloor -1)
    (return 1)
    (else
      (return distToFloor))))

(fn CheckIsBetweenGlacier
  (params (directionVec :type Vector))
  (bind _returnvalue (Transformation|GetActorLocation))
  (bind _movedistance (LocalVariables|GetmoveDistance))
  (bind _returnvalue_2 (* directionVec _movedistance))
  (bind _returnvalue_3 (+ _returnvalue_2 _returnvalue))
  (bind _returnvalue_4 (Collision|LineTraceByChannel _returnvalue_3 (+ _returnvalue_3 "0, 0,50.000000") "TraceTypeQuery1" false 0 "None" true "(R=1.000000,G=0.000000,B=0.000000,A=1.000000)" "(R=0.000000,G=1.000000,B=0.000000,A=1.000000)" 2.0))
  (if _returnvalue_4
    (return true)
    (else
      (return false))))

(fn PlayAnimwhenFall
  (params (distToFloor :type Integer))
  (if (== -1 distToFloor)
    (CallFunction|FalltoWater)
    (else
      (CallFunction|FallingSeal distToFloor))))

(fn PutSnowMesh
  (Utilities|FlowControl|Sequence
    (:then_0
      (bind _returnvalue (AddComponent|AddStaticMeshComponent false))
      (bind _output_get (Variables|Default|SetNoseSnowMesh _returnvalue))
      (Transformation|AttachComponentToComponent _output_get (Variables|Default|GetSkeletalMesh) "NoseSnowSocket" "KeepRelative" "KeepRelative" "KeepRelative" true))
    (:then_1
      (bind _returnvalue_2 (AddComponent|AddStaticMeshComponent false))
      (bind _output_get_2 (Variables|Default|SetBackSnowMesh _returnvalue_2))
      (Transformation|AttachComponentToComponent _output_get_2 (Variables|Default|GetSkeletalMesh) "BackSnowSocket" "KeepRelative" "KeepRelative" "KeepRelative" true))
    (:then_2
      (bind _returnvalue_3 (AddComponent|AddStaticMeshComponent false))
      (bind _output_get_3 (Variables|Default|SetHeadSnowMesh _returnvalue_3))
      (Transformation|AttachComponentToComponent _output_get_3 (Variables|Default|GetSkeletalMesh) "HeadSnowSocket" "KeepRelative" "KeepRelative" "KeepRelative" true))))