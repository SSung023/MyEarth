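; BP_Cormorant is a cormorant NPC that the player can chat with and that relocates between landing spots.
; Its ChatTrigger overlaps toggle the player's chat flags and cormorant reference, passing in its script DataTable on entry unless chat has ended.
; The moveNextPos event snaps the actor to the next NpcLandPos entry and advances the index.
; The turnNpc event sets mesh yaw from an eased, height-flattened look-at toward the player.
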(event OnComponentBeginOverlap(ChatTrigger)
  (params (OverlappedComponent :type Primitive%20Component%20Object%20Reference) (OtherActor :type Actor%20Object%20Reference) (OtherComp :type Primitive%20Component%20Object%20Reference) (OtherBodyIndex :type Integer) (bFromSweep :type Boolean) (SweepResult :type Hit%20Result%20Structure%20%28by%20ref%29))
  ;[1 1 1] Ready to chat
  (bind _asplayer_character (Utilities|Casting|CastToPlayerCharacter OtherActor))
  (bind _output_get (Variables|Default|Setplayer _asplayer_character))
  (Variables|/Game/Blueprints/Character/feat_player/PlayerCharacter.PlayerCharacter_C|SetisReadyToChat _output_get true)
  (if (Variables|Default|GetisChatEnd)
    _
    (else
      (Variables|/Game/Blueprints/Character/feat_player/PlayerCharacter.PlayerCharacter_C|SetscriptDT _output_get (Variables|Default|GetscriptDataTable))))
  (Variables|/Game/Blueprints/Character/feat_player/PlayerCharacter.PlayerCharacter_C|Setcormorant _output_get self))

(event OnComponentEndOverlap(ChatTrigger)
  (params (OverlappedComponent :type Primitive%20Component%20Object%20Reference) (OtherActor :type Actor%20Object%20Reference) (OtherComp :type Primitive%20Component%20Object%20Reference) (OtherBodyIndex :type Integer))
  ;[1 1 1] Ready to chat
  (bind _asplayer_character (Utilities|Casting|CastToPlayerCharacter OtherActor))
  (bind _output_get (Variables|Default|Setplayer _asplayer_character))
  (Variables|/Game/Blueprints/Character/feat_player/PlayerCharacter.PlayerCharacter_C|SetisReadyToChat _output_get false)
  (Variables|/Game/Blueprints/Character/feat_player/PlayerCharacter.PlayerCharacter_C|SetisChatting _output_get false)
  (Variables|/Game/Blueprints/Character/feat_player/PlayerCharacter.PlayerCharacter_C|Setcormorant _output_get 0))

(event Custom|turnNpc
  (bind _returnvalue (Transformation|GetActorLocation))
  (bind _player (Variables|Default|Getplayer))
  (bind (_x _y) (Math|Vector|BreakVector _returnvalue))
  (bind _returnvalue_2 (Transformation|GetActorLocation _player))
  (bind (_x_2 _y_2) (Math|Vector|BreakVector _returnvalue_2))
  ;[1 1 1] Turn npc direction
  (Transformation|SetWorldRotation (Variables|Default|GetCormorantMesh) (Math|Rotator|MakeRotator 0.0 0.0 (Math|Interpolation|Ease "EaseOut" 0.0 (.yaw (Math|Rotator|FindLookatRotation (Math|Vector|MakeVector _x _y 0.0) (Math|Vector|MakeVector _x_2 _y_2 0.0))) (.yaw (Transformation|GetActorRotation _player)) 2.0)) false false))

(event Custom|moveNextPos
  (if (> (Utilities|Array|Length (Variables|Default|GetnpcLandPos)) (Variables|Default|GetcurPosIdx))
    (Transformation|SetActorLocation (Transformation|GetActorLocation (Utilities|Array|Get(acopy) (Variables|Default|GetnpcLandPos) (Variables|Default|GetcurPosIdx))) false false)
    (if (> (Utilities|Array|Length (Variables|Default|GetnpcLandPos)) (Variables|Default|GetcurPosIdx))
      (Math|Integer|IncrementInt (Variables|Default|GetcurPosIdx)))))

(fn ConstructionScript)