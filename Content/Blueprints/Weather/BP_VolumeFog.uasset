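; BP_VolumeFog is a volumetric fog actor whose opacity can fade in and out and whose look can be changed at runtime.
; The construction script creates a dynamic material instance on the Volume, caches its initial opacity, and optionally spawns it hidden.
; FadeIn and FadeOut play one timeline forward or backward, easing opacity between zero and that cached value with an adjustable exponent.
; Low-level events instantly set opacity, any scalar parameter, color or mask texture, or restore the initial opacity.
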(event Custom|FadeOut
  ;[1 0.9677 0.4742] 기본 이벤트
  (bind _alphacurve (Timeline|Alpha ReverseFromEnd)
    (:Update
      (CallFunction|SetOpacityValueInstant (Class|KismetMathLibrary|FInterpEaseinOut 0.0 (Variables|Default|GetInitialOpacityValue) _alphacurve (Variables|Default|GetFadeSpeedEx))))))

(event Custom|FadeIn
  ;[1 0.9677 0.4742] 기본 이벤트
  (bind _alphacurve (Timeline|Alpha PlayFromStart)
    (:Update
      (CallFunction|SetOpacityValueInstant (Class|KismetMathLibrary|FInterpEaseinOut 0.0 (Variables|Default|GetInitialOpacityValue) _alphacurve (Variables|Default|GetFadeSpeedEx))))))

(event Custom|SetColorInstant
  (params (Value :type Linear%20Color%20Structure))
  ;[0.9524 0.5568 1] Low-Level 조정용 이벤트
  (Rendering|Material|SetVectorParameterValue (Variables|Default|GetFogMatInstance) "Fog Color" Value :!class /Script/Engine.MaterialInstanceDynamic))

(event Custom|ReturnOpacityInitialValue
  ;[0.9524 0.5568 1] Low-Level 조정용 이벤트
  (Rendering|Material|SetScalarParameterValue (Variables|Default|GetFogMatInstance) (Variables|Default|GetOpacityName) (Variables|Default|GetInitialOpacityValue) :!class /Script/Engine.MaterialInstanceDynamic))

(event Custom|SetTextureInstant
  (params (Value :type Texture%202D%20Object%20Reference))
  ;[0.9524 0.5568 1] Low-Level 조정용 이벤트
  (Rendering|Material|SetTextureParameterValue (Variables|Default|GetFogMatInstance) "Mask" Value))

(event Custom|SetOpacityValueInstant
  (params (Value :type Float%20%28single-precision%29))
  ;[0.9524 0.5568 1] Low-Level 조정용 이벤트
  (Rendering|Material|SetScalarParameterValue (Variables|Default|GetFogMatInstance) (Variables|Default|GetOpacityName) Value :!class /Script/Engine.MaterialInstanceDynamic))

(event Custom|SetScalarParameterInstant
  (params (Parameter%20Name :type Name) (Value :type Float%20%28single-precision%29))
  ;[0.9524 0.5568 1] Low-Level 조정용 이벤트
  (Rendering|Material|SetScalarParameterValue (Variables|Default|GetFogMatInstance) Parameter%20Name Value :!class /Script/Engine.MaterialInstanceDynamic))

(fn ConstructionScript
  (bind _returnvalue (Rendering|Material|CreateDynamicMaterialInstance (Variables|Default|GetVolume) 0 (Variables|Default|GetSourceMaterial) "None" :!class /Script/Engine.PrimitiveComponent))
  (Variables|Default|SetFogMatInstance _returnvalue)
  (Variables|Default|SetInitialOpacityValue (CallFunction|GetCurrentOpacityValue))
  (if (Variables|Default|GetSpawnHidden)
    (CallFunction|SetOpacityValueInstant 0.0)))

(fn GetCurrentOpacityValue
  (bind _returnvalue (Rendering|Material|GetScalarParameterValue (Variables|Default|GetFogMatInstance) (Variables|Default|GetOpacityName) :!class /Script/Engine.MaterialInstanceDynamic))
  (return _returnvalue))