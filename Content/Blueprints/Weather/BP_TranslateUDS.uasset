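; BP_TranslateUDS is a one-shot trigger actor that starts a time-of-day transition when the PlayerCharacter enters its TriggerVolume.
; On overlap it destroys the volume component, then finds the BP_WeatherManager through GetActorOfClass.
; It copies its transition curve, duration and next time of day into the manager, then calls SetTimeline and TranslateUDS there to run the change.
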(event OnComponentBeginOverlap(TriggerVolume)
  (params (OverlappedComponent :type Primitive%20Component%20Object%20Reference) (OtherActor :type Actor%20Object%20Reference) (OtherComp :type Primitive%20Component%20Object%20Reference) (OtherBodyIndex :type Integer) (bFromSweep :type Boolean) (SweepResult :type Hit%20Result%20Structure%20%28by%20ref%29))
  (Utilities|Casting|CastToPlayerCharacter OtherActor)
  (Components|DestroyComponent (Variables|Default|GetTriggerVolume))
  (bind _returnvalue (Actor|GetActorOfClass "/Game/Blueprints/Weather/BP_WeatherManager.BP_WeatherManager_C"))
  (Utilities|FlowControl|Sequence
    (:then_0
      (Variables|/Game/Blueprints/Weather/BP_WeatherManager.BP_WeatherManager_C|SetTransition%20Curve _returnvalue (Variables|Default|GetCurve))
      (Variables|/Game/Blueprints/Weather/BP_WeatherManager.BP_WeatherManager_C|SetTransition%20Time _returnvalue (Variables|Default|GetTransition%20Time))
      (Variables|/Game/Blueprints/Weather/BP_WeatherManager.BP_WeatherManager_C|SetNext%20Time%20of%20Day _returnvalue (Variables|Default|GetNext%20Time%20of%20Day))
      (Default|SetTimeline _returnvalue)
      (Default|TranslateUDS _returnvalue))))

(event EventBeginPlay)

(event Collision|EventActorBeginOverlap
  (params (OtherActor :type Actor%20Object%20Reference)))

(event EventTick
  (params (DeltaSeconds :type Float%20%28single-precision%29)))

(fn ConstructionScript)