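; Placeable trigger volume that changes Ultra Dynamic Sky lighting through BP_WeatherManager when the player enters.
; The Construction Script uses TriggerType to keep one of three trigger components and destroy the others.
; The one-shot aurora trigger starts an intensity transition, the view point lowers moonlight while the player's capsule is inside and raises it on exit, and the sky mode trigger switches the UDS sky mode.
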(event OnComponentBeginOverlap(AuroraTrigger)
  (params (OverlappedComponent :type Primitive%20Component%20Object%20Reference) (OtherActor :type Actor%20Object%20Reference) (OtherComp :type Primitive%20Component%20Object%20Reference) (OtherBodyIndex :type Integer) (bFromSweep :type Boolean) (SweepResult :type Hit%20Result%20Structure%20%28by%20ref%29))
  ;[1 1 1] Aurora
  (Utilities|Casting|CastToPlayerCharacter OtherActor)
  (Components|DestroyComponent (Variables|Default|GetAurora%20Trigger))
  (bind _returnvalue (Actor|GetActorOfClass "/Game/Blueprints/Weather/BP_WeatherManager.BP_WeatherManager_C"))
  (bind _output_get (Variables|Default|SetWeather%20Manager _returnvalue))
  (Variables|/Game/Blueprints/Weather/BP_WeatherManager.BP_WeatherManager_C|SetNext%20Aurora%20Intensity _output_get (Variables|Aurora|GetNext%20Aurora%20Intensity))
  (Default|TranslateAuroraIntensity _output_get))

(event OnComponentBeginOverlap(ViewPoint)
  (params (OverlappedComponent :type Primitive%20Component%20Object%20Reference) (OtherActor :type Actor%20Object%20Reference) (OtherComp :type Primitive%20Component%20Object%20Reference) (OtherBodyIndex :type Integer) (bFromSweep :type Boolean) (SweepResult :type Hit%20Result%20Structure%20%28by%20ref%29))
  ;[1 1 1] View Point
  (Utilities|Casting|CastToPlayerCharacter OtherActor)
  (Utilities|Casting|CastToCapsuleComponent OtherComp)
  (bind _returnvalue (Actor|GetActorOfClass "/Game/Blueprints/Weather/BP_WeatherManager.BP_WeatherManager_C"))
  (bind _output_get (Variables|Default|SetWeather%20Manager _returnvalue))
  (Variables|/Game/Blueprints/Weather/BP_WeatherManager.BP_WeatherManager_C|SetNext%20Moon%20Light%20Intensity _output_get 0.1)
  (Default|TranslateMoonLight _output_get))

(event OnComponentEndOverlap(ViewPoint)
  (params (OverlappedComponent :type Primitive%20Component%20Object%20Reference) (OtherActor :type Actor%20Object%20Reference) (OtherComp :type Primitive%20Component%20Object%20Reference) (OtherBodyIndex :type Integer))
  ;[1 1 1] View Point
  (Utilities|Casting|CastToPlayerCharacter OtherActor)
  (Utilities|Casting|CastToCapsuleComponent OtherComp)
  (bind _returnvalue (Actor|GetActorOfClass "/Game/Blueprints/Weather/BP_WeatherManager.BP_WeatherManager_C"))
  (bind _output_get (Variables|Default|SetWeather%20Manager _returnvalue))
  (Variables|/Game/Blueprints/Weather/BP_WeatherManager.BP_WeatherManager_C|SetNext%20Moon%20Light%20Intensity _output_get 0.2)
  (Default|TranslateMoonLight _output_get))

(event OnComponentBeginOverlap(SkyModeTrigger)
  (params (OverlappedComponent :type Primitive%20Component%20Object%20Reference) (OtherActor :type Actor%20Object%20Reference) (OtherComp :type Primitive%20Component%20Object%20Reference) (OtherBodyIndex :type Integer) (bFromSweep :type Boolean) (SweepResult :type Hit%20Result%20Structure%20%28by%20ref%29))
  (Utilities|Casting|CastToPlayerCharacter OtherActor)
  (Utilities|Casting|CastToCapsuleComponent OtherComp)
  (bind _returnvalue (Actor|GetActorOfClass "/Game/Blueprints/Weather/BP_WeatherManager.BP_WeatherManager_C"))
  (bind _output_get (Variables|Default|SetWeather%20Manager _returnvalue))
  (Default|ChangeUDSSkyMode _output_get "NewEnumerator0"))

(fn ConstructionScript
  (switch Utilities|FlowControl|Switch|SwitchonUDS_Trigger_Type (Variables|Default|GetTrigger%20Type)
    (:NewEnumerator2
      (Components|DestroyComponent (Variables|Default|GetView%20Point))
      (Components|DestroyComponent (Variables|Default|GetSky%20Mode%20Trigger)))
    (:NewEnumerator3
      (Components|DestroyComponent (Variables|Default|GetAurora%20Trigger))
      (Components|DestroyComponent (Variables|Default|GetSky%20Mode%20Trigger)))
    (:NewEnumerator1
      (Components|DestroyComponent (Variables|Default|GetView%20Point))
      (Components|DestroyComponent (Variables|Default|GetAurora%20Trigger)))))