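; BP_FlatFog is a weather actor that renders fog on a plane through a dynamic material instance.
; The construction script creates the instance, caches its initial emissive value as fog density, and zeroes it when SpawnHidden is set.
; FadeIn and FadeOut play the Alpha timeline forward or backward, easing density with a configurable exponent.
; Other events instantly set color, noise texture, density or any scalar parameter, or restore initial density.
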(event Custom|FadeOut
  ;[1 0.9677 0.4742] 기본 이벤트
  (bind _alphacurve (Timeline|Alpha ReverseFromEnd)
    (:Update
      (CallFunction|SetEmissiveValueInstant (Class|KismetMathLibrary|FInterpEaseinOut 0.0 (Variables|Default|GetInitialEmissiveValue) _alphacurve (Variables|Default|GetFadeSpeedEx))))))

(event Custom|FadeIn
  ;[1 0.9677 0.4742] 기본 이벤트
  (bind _alphacurve (Timeline|Alpha PlayFromStart)
    (:Update
      (CallFunction|SetEmissiveValueInstant (Class|KismetMathLibrary|FInterpEaseinOut 0.0 (Variables|Default|GetInitialEmissiveValue) _alphacurve (Variables|Default|GetFadeSpeedEx))))))

(event Custom|SetColorInstant
  (params (Value :type Linear%20Color%20Structure))
  ;[0.5207 0.6616 1] Low-Level 조정용 이벤트
  (Rendering|Material|SetVectorParameterValue (Variables|Default|GetFogMatInstance) "Color" Value :!class /Script/Engine.MaterialInstanceDynamic))

(event Custom|ReturnEmissiveInitialValue
  ;[0.5207 0.6616 1] Low-Level 조정용 이벤트
  (Rendering|Material|SetScalarParameterValue (Variables|Default|GetFogMatInstance) (Variables|Default|GetEmissive%20Name) (Variables|Default|GetInitialEmissiveValue) :!class /Script/Engine.MaterialInstanceDynamic))

(event Custom|SetTextureInstant
  (params (Value :type Texture%202D%20Object%20Reference))
  ;[0.5207 0.6616 1] Low-Level 조정용 이벤트
  (Rendering|Material|SetTextureParameterValue (Variables|Default|GetFogMatInstance) "Noise Texture" Value))

(event Custom|SetEmissiveValueInstant
  (params (Value :type Float%20%28single-precision%29))
  ;[0.5207 0.6616 1] Low-Level 조정용 이벤트
  (Rendering|Material|SetScalarParameterValue (Variables|Default|GetFogMatInstance) (Variables|Default|GetEmissive%20Name) Value :!class /Script/Engine.MaterialInstanceDynamic))

(event Custom|SetScalarParameterInstant
  (params (Parameter%20Name :type Name) (Value :type Float%20%28single-precision%29))
  ;[0.5207 0.6616 1] Low-Level 조정용 이벤트
  (Rendering|Material|SetScalarParameterValue (Variables|Default|GetFogMatInstance) Parameter%20Name Value :!class /Script/Engine.MaterialInstanceDynamic))

(fn ConstructionScript
  (bind _returnvalue (Rendering|Material|CreateDynamicMaterialInstance (Variables|Default|GetPlane) 0 (Variables|Default|GetSource%20Material) "None" :!class /Script/Engine.PrimitiveComponent))
  (Variables|Default|SetFogMatInstance _returnvalue)
  (Variables|Default|SetInitialEmissiveValue (CallFunction|GetCurrentEmissiveValue))
  (if (Variables|Default|GetSpawnHidden)
    (CallFunction|SetEmissiveValueInstant 0.0)))

(fn GetCurrentEmissiveValue
  (bind _returnvalue (Rendering|Material|GetScalarParameterValue (Variables|Default|GetFogMatInstance) (Variables|Default|GetEmissive%20Name) :!class /Script/Engine.MaterialInstanceDynamic))
  (return _returnvalue))