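; BP_water is a water hazard that respawns the player character on contact with its overlap collider.
; It moves a camera actor, assigned through setNewCamera, to the current view and blends to it, leaving the view detached from the player.
; It then flags the player as respawning, plays a slowed penguin in-water montage, fades the screen out and calls WrapToGround on the character.
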(event OnComponentBeginOverlap(overlapcollider)
  (params (OverlappedComponent :type Primitive%20Component%20Object%20Reference) (OtherActor :type Actor%20Object%20Reference) (OtherComp :type Primitive%20Component%20Object%20Reference) (OtherBodyIndex :type Integer) (bFromSweep :type Boolean) (SweepResult :type Hit%20Result%20Structure%20%28by%20ref%29))
  (bind _returnvalue (Game|GetPlayerCameraManager 0))
  (if (Actor|ActorHasTag OtherActor "Player")
    (Transformation|SetActorLocationAndRotation (Variables|Default|GetnewCamera) (Camera|GetCameraLocation _returnvalue) (Camera|GetCameraRotation _returnvalue))
    (Game|Player|SetViewTargetwithBlend (Game|GetPlayerController 0) (Variables|Default|GetnewCamera) 0.5 "VTBlend_Linear" 0.0 false)
    (CallFunction|DisablePlayer)
    (CallFunction|FadeOutandWrap)))

(event Custom|setNewCamera
  (params (NewParam :type Object%20Object%20Reference))
  (bind _ascamera_actor (Utilities|Casting|CastToCameraActor NewParam))
  (Variables|Default|SetnewCamera _ascamera_actor))

(event Custom|disablePlayer
  (bind _asplayer_character (Utilities|Casting|CastToPlayerCharacter (Game|GetPlayerCharacter 0)))
  (Variables|/Game/Blueprints/Character/feat_player/PlayerCharacter.PlayerCharacter_C|SetisRespawning _asplayer_character true)
  (Animation|Montage|PlayMontage (Variables|/Game/Blueprints/Character/feat_player/PlayerCharacter.PlayerCharacter_C|GetPenguinSkeletal _asplayer_character) "/Game/Blueprints/Character/feat_player/montage/MT_penguin_jump.MT_penguin_jump" 0.3 0.0 "inWater"))

(event Custom|fadeOutAndWrap
  (Utilities|FlowControl|Delay 1.0)
  (CameraFades|StartCameraFade :self (Game|GetPlayerCameraManager 0) :ToAlpha 1.0 :Duration 1.0 :bHoldWhenFinished true)
  (Utilities|FlowControl|Delay 1.0)
  (Default|WraptoGround (stale Custom|disablePlayer _asplayer_character)))

(fn ConstructionScript)