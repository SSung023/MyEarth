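; BP_WeatherManager drives smooth transitions of Ultra Dynamic Sky's time of day, aurora intensity and moon light intensity.
; BeginPlay caches the sky and weather actors, though only the sky is modified.
; Each Translate event snapshots the current value and eases toward its Next variable on a timeline, stopping and restarting if already playing.
; Setter events adjust the time-of-day curve and length and the aurora length; debug prints report results.
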(event Custom|Translate%20Aurora%20Intensity
  ;[1 1 1] Change Aurora Intensity
  (if (not (Audio|Components|Audio|IsPlaying (Variables|Default|GetAurora%20Transition)))
    (Variables|Aurora|SetPrev%20Aurora%20Intensity (Variables|/Game/UltraDynamicSky/Blueprints/Ultra_Dynamic_Sky.Ultra_Dynamic_Sky_C|GetAurora%20Intensity (Variables|Default|GetUDS)))
    (bind _alpha (Timeline|Aurora%20Transition PlayFromStart)
      (:Update
        (Variables|/Game/UltraDynamicSky/Blueprints/Ultra_Dynamic_Sky.Ultra_Dynamic_Sky_C|SetAurora%20Intensity (Variables|Default|GetUDS) (Math|Interpolation|Ease "EaseOut" _alpha (Variables|Aurora|GetPrev%20Aurora%20Intensity) (Variables|Aurora|GetNext%20Aurora%20Intensity) 2.0))))
    (else
      (Utilities|FlowControl|Sequence
        (:then_0
          (Timeline|Aurora%20Transition Stop))
        (:then_1
          (CallFunction|TranslateAuroraIntensity))))))

(event Custom|Translate%20TIme
  ;[1 1 1] Change Time
  (if (not (Audio|Components|Audio|IsPlaying (Variables|Default|GetTime%20of%20Day%20Transition)))
    (bind _time (Default|GetTimeOfDayinRealTimeFormat (Variables|Default|GetUDS)))
    (bind _output_get (Variables|Default|SetPrev%20Timecode _time))
    (Development|PrintString (Class|TimeManagementBlueprintLibrary|ToString(Timecode) _output_get false) true false)
    (bind _alpha (Timeline|Time%20of%20Day%20Transition PlayFromStart)
      (:Update
        (bind _timeofday (CallFunction|GetTimeOfDayUsingTimeCode (Variables|Default|GetPrev%20Timecode)))
        (bind _timecode (CallFunction|ConvertTimeOfDaytoTimeCode (Math|Interpolation|Ease "EaseOut" _alpha _timeofday (Variables|Default|GetNext%20Time%20of%20Day) 2.0)))
        (Default|SetTimeOfDayUsingTimeCode (Variables|Default|GetUDS) _timecode))
      (:Finished
        (bind _time_2 (Default|GetTimeOfDayinRealTimeFormat (Variables|Default|GetUDS)))
        (Development|PrintString (Class|TimeManagementBlueprintLibrary|ToString(Timecode) _time_2 false) true false)
        (bind _timeofday_2 (CallFunction|GetTimeOfDayUsingTimeCode _time_2))
        (Development|PrintString (Utilities|String|ToString(Float) _timeofday_2) true false)))
    (else
      (Utilities|FlowControl|Sequence
        (:then_0
          (Timeline|Time%20of%20Day%20Transition Stop))
        (:then_1
          (CallFunction|TranslateTIme))))))

(event Custom|Set%20Time%20of%20Day%20Timeline
  (bind _time_of_day_transition (Variables|Default|GetTime%20of%20Day%20Transition))
  ;[1 1 1] Time of Day Timeline Setter
  (Class|TimelineComponent|SetFloatCurve _time_of_day_transition (Variables|Timeline|GetTransition%20Curve) "Alpha")
  (Components|Timeline|SetTimelineLength _time_of_day_transition (Variables|Timeline|GetTransition%20Time)))

(event Custom|Set%20Aurora%20Timeline
  ;[1 1 1] Aurora Timeline Setter
  (Components|Timeline|SetTimelineLength (Variables|Default|GetAurora%20Transition) (Variables|Aurora|GetAurora%20Transition%20Time)))

(event Custom|Translate%20Moon%20Light
  ;[1 1 1] Change Moon Light Intensity
  (if (not (Audio|Components|Audio|IsPlaying (Variables|Default|GetMoon%20Light%20Transition)))
    (Variables|MoonLight|SetPrev%20Moon%20Light%20Intensity (Variables|/Game/UltraDynamicSky/Blueprints/Ultra_Dynamic_Sky.Ultra_Dynamic_Sky_C|GetMoon%20Light%20Intensity (Variables|Default|GetUDS)))
    (bind _alpha (Timeline|Moon%20Light%20Transition PlayFromStart)
      (:Update
        (Variables|/Game/UltraDynamicSky/Blueprints/Ultra_Dynamic_Sky.Ultra_Dynamic_Sky_C|SetMoon%20Light%20Intensity (Variables|Default|GetUDS) (Math|Interpolation|Ease "EaseInOut" _alpha (Variables|MoonLight|GetPrev%20Moon%20Light%20Intensity) (Variables|MoonLight|GetNext%20Moon%20Light%20Intensity) 2.0)))
      (:Finished
        (Development|PrintString (Utilities|String|ToString(Float) (Variables|/Game/UltraDynamicSky/Blueprints/Ultra_Dynamic_Sky.Ultra_Dynamic_Sky_C|GetMoon%20Light%20Intensity (Variables|Default|GetUDS))))))
    (else
      (Utilities|FlowControl|Sequence
        (:then_0
          (Timeline|Moon%20Light%20Transition Stop))
        (:then_1
          (CallFunction|TranslateMoonLight))))))

(event EventBeginPlay
  ;[1 1 1] Initial Setting
  (bind _returnvalue (Actor|GetActorOfClass "/Game/UltraDynamicSky/Blueprints/Ultra_Dynamic_Sky.Ultra_Dynamic_Sky_C"))
  (Variables|Default|SetUDS _returnvalue)
  (bind _returnvalue_2 (Actor|GetActorOfClass "/Game/UltraDynamicSky/Blueprints/Ultra_Dynamic_Weather.Ultra_Dynamic_Weather_C"))
  (Variables|Default|SetUDW _returnvalue_2))

(fn ConstructionScript)