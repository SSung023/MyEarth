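; Blueprint function library that prints tagged, timestamped playtest event lines for respawns, save points, glacier pushes, seal incidents and killer whale launches.
; Each logger formats time, level and event objects into PrintString, most adding the submap from PlayerGameMode.
; Respawn and glacier lines go only to the log, seal and whale lines only to screen, save points to both.
; Submap entry/exit prints are unreachable, and the jump logger is empty.
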(fn GetNowasText
  (return (Utilities|String|ToString(Text) (Utilities|Text|FormatText "[{string}]" (Class|KismetTextLibrary|AsDateTimeDateTime (Math|DateTime|Now))))))

(fn LoggingSubmapEntry
  (params (Level%20Name :type String))
  (bind _now (CallFunction|GetNowasText))
  (bind _returnvalue (Game|GetCurrentLevelName 0)))

(fn LoggingSubmapExit
  (params (Level%20Name :type String))
  (bind _now (CallFunction|GetNowasText))
  (bind _returnvalue (Game|GetCurrentLevelName 0)))

(fn LoggingRespawn
  (bind _now (CallFunction|GetNowasText))
  (bind _asplayer_game_mode (Utilities|Casting|CastToPlayerGameMode (Game|GetGameMode))
    (:then
      _)
    (:CastFailed
      _))
  (bind _returnvalue (Game|GetCurrentLevelName 0))
  (Development|PrintString 0 (Utilities|String|ToString(Text) (Utilities|Text|FormatText "[Respawn] \"{when}\" \"{level}\" \"{submap}\" \"{respawn obj}\" \"{string}\"" _now _returnvalue (Variables|/Game/Blueprints/Character/feat_system/PlayerGameMode.PlayerGameMode_C|GetlevelName _asplayer_game_mode) (Utilities|GetDisplayName (Variables|/Game/Blueprints/Character/feat_system/PlayerGameMode.PlayerGameMode_C|GetrespawnObj _asplayer_game_mode)) (Utilities|Text|ToText(String) "리스폰 실행"))) false true "(R=0.000000,G=0.660000,B=1.000000,A=1.000000)" 1e+01))

(fn LoggingSavePoint
  (params (Level%20Name :type String) (Respawn%20Object :type Actor%20Object%20Reference))
  (bind _now (CallFunction|GetNowasText))
  (bind _returnvalue (Game|GetCurrentLevelName 0))
  (Development|PrintString 0 (Utilities|String|ToString(Text) (Utilities|Text|FormatText "[PlayTime] \"{when}\" \"{who}\" \"{level}\" \"{submap}\" \"{what}\"" _now (Utilities|GetDisplayName "/Game/Blueprints/Character/feat_player/PlayerCharacter.PlayerCharacter") _returnvalue Level%20Name (Utilities|String|Append (Utilities|GetDisplayName Respawn%20Object) " " "통과"))) true true "(R=0.000000,G=0.660000,B=1.000000,A=1.000000)" 15.0))

(fn LoggingGlacierPush
  (params (Glacier%20Obj :type Actor%20Object%20Reference))
  (bind _now (CallFunction|GetNowasText))
  (bind _asplayer_game_mode (Utilities|Casting|CastToPlayerGameMode (Game|GetGameMode))
    (:then
      _)
    (:CastFailed
      _))
  (bind _returnvalue (Game|GetCurrentLevelName 0))
  (Development|PrintString 0 (Utilities|String|ToString(Text) (Utilities|Text|FormatText "[Glacier] \"{when}\" \"{level}\" \"{submap}\" \"{respawn obj}\" \"{string}\"" _now _returnvalue (Variables|/Game/Blueprints/Character/feat_system/PlayerGameMode.PlayerGameMode_C|GetlevelName _asplayer_game_mode) (Utilities|GetDisplayName (Variables|/Game/Blueprints/Character/feat_system/PlayerGameMode.PlayerGameMode_C|GetrespawnObj _asplayer_game_mode)) (Utilities|String|Append (Utilities|GetDisplayName Glacier%20Obj) " 밀림"))) false true "(R=0.000000,G=0.660000,B=1.000000,A=1.000000)" 1e+01))

(fn LoggingPlayerJump)

(fn LoggingSealFalltoWater
  (params (Seal%20Obj :type BP%20Seals%20Object%20Reference))
  (bind _now (CallFunction|GetNowasText))
  (bind _asplayer_game_mode (Utilities|Casting|CastToPlayerGameMode (Game|GetGameMode)))
  (bind _returnvalue (Game|GetCurrentLevelName 0))
  (Development|PrintString 0 (Utilities|String|ToString(Text) (Utilities|Text|FormatText "[Seal] \"{when}\" \"{level}\" \"{submap}\" \"{seal obj}\" \"{action}\"" _now _returnvalue (Variables|/Game/Blueprints/Character/feat_system/PlayerGameMode.PlayerGameMode_C|GetlevelName _asplayer_game_mode) (Utilities|GetDisplayName Seal%20Obj) (Utilities|Text|ToText(String) "Fall To Water"))) true false "(R=0.000000,G=0.660000,B=1.000000,A=1.000000)" 1e+01))

(fn LoggingSnowySeal
  (params (Seal%20Obj :type BP%20Seals%20Object%20Reference))
  (bind _now (CallFunction|GetNowasText))
  (bind _asplayer_game_mode (Utilities|Casting|CastToPlayerGameMode (Game|GetGameMode)))
  (bind _returnvalue (Game|GetCurrentLevelName 0))
  (Development|PrintString 0 (Utilities|String|ToString(Text) (Utilities|Text|FormatText "[Seal] \"{when}\" \"{level}\" \"{submap}\" \"{seal obj}\" \"{action}\"" _now _returnvalue (Variables|/Game/Blueprints/Character/feat_system/PlayerGameMode.PlayerGameMode_C|GetlevelName _asplayer_game_mode) (Utilities|GetDisplayName Seal%20Obj) (Utilities|Text|ToText(String) "Snowy Seal"))) true false "(R=0.000000,G=0.660000,B=1.000000,A=1.000000)" 1e+01))

(fn LoggingKillerWhaleLaunch
  (params (KillerWhale%20Obj :type BP%20Killer%20Whale%20Object%20Reference))
  (bind _now (CallFunction|GetNowasText))
  (bind _asplayer_game_mode (Utilities|Casting|CastToPlayerGameMode (Game|GetGameMode)))
  (bind _returnvalue (Game|GetCurrentLevelName 0))
  (Development|PrintString 0 (Utilities|String|ToString(Text) (Utilities|Text|FormatText "[KillerWhale] \"{when}\" \"{level}\" \"{submap}\" \"{killerwhale obj}\" \"{action}\"" _now _returnvalue (Variables|/Game/Blueprints/Character/feat_system/PlayerGameMode.PlayerGameMode_C|GetlevelName _asplayer_game_mode) (Utilities|GetDisplayName KillerWhale%20Obj) (Utilities|Text|ToText(String) "Launch"))) true false "(R=0.000000,G=0.660000,B=1.000000,A=1.000000)" 1e+01))