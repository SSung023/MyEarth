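; FL_UDS is a function library that converts between clock time or Timecode and a float Time of Day with 100 units per hour.
; Hours, minutes, seconds and milliseconds are scaled and summed, with the sub-minute part clamped to one minute.
; The reverse splits the float with nested Floor and Fraction calls.
; Timecode conversions assume 60 frames per second, and Timecode input reuses the clock-time function.
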(fn H/M/S/MStoTimeOfDay
  (params (Hours :type Integer) (Minutes :type Integer) (Seconds :type Integer) (Miliseconds :type Integer))
  (bind _returnvalue (/ 1e+02 6e+01))
  (return (+ (+ (* (Math|Conversions|ToFloat(Integer) Hours) 1e+02) (* (Math|Conversions|ToFloat(Integer) Minutes) _returnvalue)) (Math|Float|MapRangeClamped (+ (Math|Conversions|ToFloat(Integer) Seconds) (/ (Math|Conversions|ToFloat(Integer) Miliseconds) 1e+03)) 0.0 6e+01 0.0 _returnvalue))))

(fn ConvertTimeOfDaytoTimeCode
  (params (Time :type Float%20%28single-precision%29))
  (bind _returnvalue (/ Time 1e+02))
  (bind _returnvalue_2 (Math|Float|Fraction _returnvalue))
  (bind _returnvalue_3 (* _returnvalue_2 6e+01))
  (bind _returnvalue_4 (Math|Float|Fraction _returnvalue_3))
  (bind _returnvalue_5 (* _returnvalue_4 6e+01))
  (return (Utilities|Struct|MakeTimecode (Math|Float|Floor _returnvalue) (Math|Float|Floor _returnvalue_3) (Math|Float|Floor _returnvalue_5) (Math|Float|Floor (* (Math|Float|Fraction _returnvalue_5) 6e+01)))))

(fn GetTimeOfDayUsingTimeCode
  (params (Timecode :type Timecode%20Structure))
  (bind (_hours _minutes _seconds _frames) (Utilities|Struct|BreakTimecode Timecode))
  (bind _time (CallFunction|H/M/S/MStoTimeOfDay _hours _minutes _seconds (Math|Float|Truncate (* (Math|Conversions|ToFloat(Integer) _frames) 16.66))))
  (return _time))