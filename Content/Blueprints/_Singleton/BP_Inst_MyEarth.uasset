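; MyEarth singleton Blueprint (apparently the game instance) that acts as the background music manager.
; Play, stop and change events drive one stored 2D audio component that persists across level transitions, using fades for transitions.
; A SetMusicPlay flag gates playback, and its toggle fades the current track in as a temporary solution or out instantly.
; Sound-mix volume override nodes are present but unconnected.
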(event Custom|Fade%20out
  (params (Fade-out%20Duration :type Float%20%28single-precision%29))
  ;[0.7894 1 0.1357] Music Manager
  ;;[1 1 1] Fade out
  (bind _output_get (Variables|MusicManager|SetFade-out%20Duration Fade-out%20Duration))
  (Audio|Components|Audio|FadeOut (Variables|Default|GetBGM%20Instance) _output_get 0.0 "Linear" :!class /Script/Engine.AudioComponent))

(event Custom|ToggleMusic
  (params (SetMusicPlay :type Boolean))
  ;[0.7894 1 0.1357] Music Manager
  (bind _output_get (Variables|Default|SetSet%20Music%20Play SetMusicPlay))
  (if _output_get
    ;;[1 0.2207 0.3305] Temporary solution
    (Audio|Components|Audio|FadeIn (Variables|Default|GetBGM%20Instance) 0.0 1.0 0.0 "Linear" :!class /Script/Engine.AudioComponent)
    (else
      (CallFunction|FadeOut 0.0))))

(event EventPlayBGM
  (params (BGM%20to%20Play :type Sound%20Cue%20Object%20Reference) (FadeIn :type Float%20%28single-precision%29))
  ;[0.7894 1 0.1357] Music Manager
  ;;[1 1 1] Play Music
  (Variables|MusicManager|SetFade-in%20Duration FadeIn)
  (bind _output_get (Variables|MusicManager|SetMusic%20to%20Play BGM%20to%20Play))
  (bind _returnvalue (Audio|CreateSound2D _output_get 1.0 1.0 0.0 0 true false))
  (bind _output_get_2 (Variables|Default|SetBGM%20Instance _returnvalue))
  (if (Variables|Default|GetSet%20Music%20Play)
    (Audio|Components|Audio|FadeIn _output_get_2 (Variables|MusicManager|GetFade-in%20Duration) 1.0 0.0 "Linear" :!class /Script/Engine.AudioComponent)))

(event EventStopBGM
  (params (FadeOut :type Float%20%28single-precision%29))
  ;[0.7894 1 0.1357] Music Manager
  ;;[1 1 1] Stop Music
  (CallFunction|FadeOut FadeOut)
  (Audio|Components|Audio|StopDelayed (Variables|Default|GetBGM%20Instance) FadeOut))

(event EventChangeBGM
  (params (BGM%20to%20Play :type Sound%20Cue%20Object%20Reference) (FadeOut :type Float%20%28single-precision%29) (FadeIn :type Float%20%28single-precision%29))
  ;[0.7894 1 0.1357] Music Manager
  ;;[1 1 1] Change Music
  (CallFunction|FadeOut FadeOut)
  (CallFunction|PlayBGM BGM%20to%20Play FadeIn))