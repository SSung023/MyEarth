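; BP_DummyGlacierBrush is a construction-script brush that fills a box with a 3D grid of child actor blocks, apparently as placeholder glacier geometry.
; It first snaps the actor's X and Y to a 50-unit grid through MakeLocationSnap, leaving Z untouched.
; Nested loops then derive counts from Endpoint and BlockSize, adding child actors at block spacing, raised half a block in Z.
; The event graph holds no active logic.
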(event EventBeginPlay)

(event Collision|EventActorBeginOverlap
  (params (OtherActor :type Actor%20Object%20Reference)))

(event EventTick
  (params (DeltaSeconds :type Float%20%28single-precision%29)))

(fn ConstructionScript
  (bind _returnvalue (Transformation|GetActorLocation))
  (bind _endpoint (Variables|Default|GetEndpoint))
  (bind _blocksize (Variables|Default|GetBlockSize))
  (Variables|Default|SetHalfBlockSize (Math|Conversions|ToFloat(Integer) (/ (Variables|Default|GetBlockSize) 2)))
  (bind _result (CallFunction|MakeLocationSnap (.x _returnvalue)))
  (bind _result_2 (CallFunction|MakeLocationSnap (.y _returnvalue)))
  (Transformation|SetActorLocation (Math|Vector|MakeVector _result _result_2 (.z _returnvalue)) false false)
  (Variables|Default|SetXCount (/ (Math|Float|Round (.x _endpoint)) _blocksize))
  (Variables|Default|SetYCount (/ (Math|Float|Round (.y _endpoint)) _blocksize))
  (Variables|Default|SetZCount (/ (Math|Float|Round (+ (.z _endpoint) (Variables|Default|GetHalfBlockSize))) _blocksize))
  (for _index (range 0 (Variables|Default|GetXCount))
    (for _index_2 (range 0 (Variables|Default|GetYCount))
      (for _index_3 (range 0 (Variables|Default|GetZCount))
        (AddComponent|AddChildActorComponent false (Math|Transform|MakeTransform (Math|Vector|MakeVector (Math|Conversions|ToFloat(Integer) (* _index (Variables|Default|GetBlockSize))) (Math|Conversions|ToFloat(Integer) (* _index_2 (Variables|Default|GetBlockSize))) (+ (Math|Conversions|ToFloat(Integer) (* _index_3 (Variables|Default|GetBlockSize))) (Variables|Default|GetHalfBlockSize)))))))))

(fn MakeLocationSnap
  (params (Axis :type Float%20%28single-precision%29))
  (bind _returnvalue (Math|Float|%(Float) Axis 5e+01))
  (if (== _returnvalue 0.0)
    (LocalVariables|SetSnappedAxis Axis)
    (else
      (LocalVariables|SetRemains _returnvalue)
      (if (> (Math|Float|Absolute(Float) (LocalVariables|GetRemains)) 25.0)
        (LocalVariables|SetCompensator (- 5e+01 (LocalVariables|GetRemains)))
        (else
          (LocalVariables|SetCompensator (* (LocalVariables|GetRemains) -1.0))))
      (LocalVariables|SetSnappedAxis (+ Axis (LocalVariables|GetCompensator)))))
  (return (LocalVariables|GetSnappedAxis)))