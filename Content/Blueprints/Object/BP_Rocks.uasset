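; BP_Rocks is a procedural scatter actor that places random rock meshes over a flat area.
; Its construction script scales the RenderArea box by Distance in X and Y, flattens Z, then adds Number static mesh components with meshes picked from Rocks.
; Random points use the box's world location but serve as relative transforms, and are unseeded, so each reconstruction reshuffles them.
; The event graph has no active logic.
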(event EventBeginPlay)

(event Collision|EventActorBeginOverlap
  (params (OtherActor :type Actor%20Object%20Reference)))

(event EventTick
  (params (DeltaSeconds :type Float%20%28single-precision%29)))

(fn ConstructionScript
  (bind _distance (Variables|Default|Getdistance))
  (bind _render_area (Variables|Default|GetRender%20Area))
  (bind _rocks (Variables|Default|GetRocks))
  (Transformation|SetRelativeScale3D (Variables|Default|GetRender%20Area) (Math|Vector|MakeVector _distance _distance 0.0))
  (for _index (range 1 (Variables|Default|Getnumber))
    (bind _returnvalue (AddComponent|AddStaticMeshComponent false (Math|Transform|MakeTransform (Math|Random|RandomPointinBoundingBox (Transformation|GetWorldLocation _render_area) (Components|Box|GetScaledBoxExtent _render_area)) "0, 0, 0" "1,1,1")))
    (Components|StaticMesh|SetStaticMesh _returnvalue (Utilities|Array|Get(acopy) _rocks (Math|Random|RandomIntegerinRange 0 (Utilities|Array|LastIndex _rocks))))))