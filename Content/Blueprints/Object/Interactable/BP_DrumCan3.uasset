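; BP_DrumCan3 is an interactable drum can that gets shoved away from the player when used.
; Interact calls PlayInteraction, which applies a strong impulse to the static mesh along the player pawn's forward vector, at a raised point computed from the mesh's relative location.
; A DoOnce followed by a one-second delayed reset limits repeat shoves.
; Interact also calls PlaySound, whose event is empty here.
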(event Custom|PlaySound)

(event Custom|PlayInteraction
  (bind _staticmesh (Variables|Default|GetStaticMesh))
  (Utilities|FlowControl|DoOnce false :!label _label
    (:Completed
      (Physics|AddImpulseatLocation _staticmesh (* (Transformation|GetActorForwardVector (Game|Player|GetPlayerPawn 0)) 18000) (+ (Variables|/Script/Engine.SceneComponent|GetRelativeLocation _staticmesh) "0, 0,90.000000") "None")
      (Utilities|FlowControl|Delay 1.0)
      (goto _label Reset))))

(event EventBeginPlay)

(event Collision|EventActorBeginOverlap
  (params (OtherActor :type Actor%20Object%20Reference)))

(event EventTick
  (params (DeltaSeconds :type Float%20%28single-precision%29)))

(event EventInteract
  (CallFunction|PlayInteraction)
  (CallFunction|PlaySound))

(fn ConstructionScript)