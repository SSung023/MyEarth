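; BP_Plastic3_2 is an interactable physics prop that gets knocked away in the player pawn's forward direction on Interact.
; PlayInteraction lifts the BoxCollision constraint mode, applies an impulse to the StaticMesh at a point raised from its relative location, then restores the default constraint after a short delay.
; A DoOnce, reset after that delay, blocks repeat triggers, and the PlaySound event is an empty stub.
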(event Custom|PlayInteraction
  (bind _staticmesh (Variables|Default|GetStaticMesh))
  (Utilities|FlowControl|DoOnce false :!label _label
    (:Completed
      (Class|PrimitiveComponent|SetConstraintMode (Variables|Default|GetBoxCollision) "None")
      (Physics|AddImpulseatLocation _staticmesh (* (Transformation|GetActorForwardVector (Game|Player|GetPlayerPawn 0)) 4000) (+ (Variables|/Script/Engine.SceneComponent|GetRelativeLocation _staticmesh) "0, 0,30.000000") "None")
      (Utilities|FlowControl|Delay 0.8)
      (Class|PrimitiveComponent|SetConstraintMode (Variables|Default|GetBoxCollision) "Default")
      (goto _label Reset))))

(event Custom|PlaySound)

(event EventBeginPlay)

(event Collision|EventActorBeginOverlap
  (params (OtherActor :type Actor%20Object%20Reference)))

(event EventTick
  (params (DeltaSeconds :type Float%20%28single-precision%29)))

(event EventInteract
  (CallFunction|PlayInteraction)
  (CallFunction|PlaySound))

(fn ConstructionScript)