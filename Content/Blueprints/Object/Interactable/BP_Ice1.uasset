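; Interactable ice object that makes the player penguin play a sliding animation when Interact is triggered.
; BeginPlay caches the player character and its penguin skeletal mesh, and Interact plays one of two sliding montages chosen by a WalkSpeed threshold.
; A DoOnce gate blocks retriggering and resets only when the montage completes.
; The PlaySound event is called on interaction but has no implementation here.
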(event Custom|PlayInteract
  (bind _penguin_skeletal (Variables|Default|GetPenguin%20Skeletal))
  (Utilities|FlowControl|DoOnce false :!label _label
    (:Completed
      (if (<= (Variables|/Game/Blueprints/Character/feat_player/PlayerCharacter.PlayerCharacter_C|GetwalkSpeed (Variables|Default|GetPlayerCharacter)) 3.8e+02)
        (Animation|Montage|PlayMontage _penguin_skeletal "/Game/Blueprints/Character/feat_player/montage/MT_penguin_sliding.MT_penguin_sliding" 1.0 0.0 "Default"
          (:OnCompleted
            (goto _label Reset)))
        (else
          (Animation|Montage|PlayMontage _penguin_skeletal "/Game/Blueprints/Character/feat_player/montage/MT_penguin_sliding2.MT_penguin_sliding2" 1.0 0.0 "Default"
            (:OnCompleted
              (goto _label Reset))))))))

(event Custom|PlaySound)

(event EventBeginPlay
  (bind _asplayer_character (Utilities|Casting|CastToPlayerCharacter (Game|GetPlayerCharacter 0)))
  (bind _output_get (Variables|Default|SetPlayerCharacter _asplayer_character))
  (Variables|Default|SetPenguin%20Skeletal (Variables|/Game/Blueprints/Character/feat_player/PlayerCharacter.PlayerCharacter_C|GetPenguinSkeletal _output_get)))

(event Collision|EventActorBeginOverlap
  (params (OtherActor :type Actor%20Object%20Reference)))

(event EventTick
  (params (DeltaSeconds :type Float%20%28single-precision%29)))

(event EventInteract
  (CallFunction|PlayInteract)
  (CallFunction|PlaySound))

(fn ConstructionScript)