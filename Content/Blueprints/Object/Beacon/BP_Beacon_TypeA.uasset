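; BP_Beacon_TypeA is a beacon object whose plane can flicker its emissive glow.
; The construction script creates a dynamic instance of MI_Beacon on the plane.
; On BeginPlay, if Flickering is enabled, it stores the base Emissive value and starts the Flicker timeline.
; Each timeline update sets Emissive to that base plus the curve value scaled by FlickeringPower.
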(event Custom|DoFlicker
  (bind _value (Timeline|Flicker PlayFromStart)
    (:Update
      (Rendering|Material|SetScalarParameterValue (Variables|Material|GetMaterialInst) "Emissive" (+ (* _value (Variables|Option|GetFlickeringPower)) (Variables|Material|GetInitialEmissive)) :!class /Script/Engine.MaterialInstanceDynamic))))

(event EventBeginPlay
  (if (Variables|Option|GetFlickering)
    (bind _returnvalue (Rendering|Material|GetScalarParameterValue (Variables|Material|GetMaterialInst) "Emissive" :!class /Script/Engine.MaterialInstanceDynamic))
    (Variables|Material|SetInitialEmissive _returnvalue)
    (CallFunction|DoFlicker)))

(fn ConstructionScript
  (bind _returnvalue (Rendering|Material|CreateDynamicMaterialInstance (Variables|Default|GetPlane) 0 "/Game/Resources/beacon/MI_Beacon.MI_Beacon" "None" :!class /Script/Engine.PrimitiveComponent))
  (Variables|Material|SetMaterialInst _returnvalue))