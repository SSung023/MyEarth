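; Beacon unit Blueprint (Type B) that can flicker the emissive glow of its plane mesh.
; Construction creates a dynamic material on the plane from a source instance.
; When flickering is enabled, BeginPlay caches the initial Emissive value and plays a timeline that adds a scaled curve to it.
; An uncalled 50-unit snap helper tests a constant zero, so it never applies compensation.
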(event Custom|DoFlicker
  (bind _value (Timeline|Flicker PlayFromStart)
    (:Update
      (Rendering|Material|SetScalarParameterValue (Variables|Material|GetMaterialInst) "Emissive" (+ (* _value (Variables|Option|GetFlickeringPower)) (Variables|Material|GetInitialEmissive)) :!class /Script/Engine.MaterialInstanceDynamic))))

(event EventBeginPlay
  (if (Variables|Option|GetFlickering)
    (bind _returnvalue (Rendering|Material|GetScalarParameterValue (Variables|Material|GetMaterialInst) "Emissive" :!class /Script/Engine.MaterialInstanceDynamic))
    (Variables|Material|SetInitialEmissive _returnvalue)
    (CallFunction|DoFlicker)))

(fn ConstructionScript
  (bind _returnvalue (Rendering|Material|CreateDynamicMaterialInstance (Variables|Default|GetPlane) 0 (Variables|Material|GetSource%20Material%20Instance) "None" :!class /Script/Engine.PrimitiveComponent))
  (Variables|Material|SetMaterialInst _returnvalue))

(fn MakeLocationSnap
  (params (Axis :type Float%20%28single-precision%29))
  (bind _returnvalue (Math|Float|%(Float) 0.0 5e+01))
  (if (== _returnvalue 0.0)
    (LocalVariables|SetSnappedAxis Axis)
    (return 0.0)
    (else
      (LocalVariables|SetRemains _returnvalue)
      (if (> (Math|Float|Absolute(Float) (LocalVariables|GetRemains)) 25.0)
        (LocalVariables|SetCompensator (- 5e+01 (LocalVariables|GetRemains)))
        (else
          (LocalVariables|SetCompensator (* (LocalVariables|GetRemains) -1.0))))
      (LocalVariables|SetSnappedAxis (+ Axis (LocalVariables|GetCompensator))))))