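; BP_Z9inLogo is a space object actor that animates a logo mesh along a spline path.
; The construction script places the mesh at the spline's first point.
; On BeginPlay, the Progress timeline plays and its value is lerped over the spline length, setting the mesh's local position and rotation along the path without using spline scale.
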(event EventBeginPlay
  (bind _progressvalue (Timeline|Progress Play)
    (:Update
      (Transformation|SetRelativeTransform (Variables|Default|GetLogoMesh) (Spline|GetTransformatDistanceAlongSpline (Variables|Default|GetSpline) (Math|Float|Lerp 0.0 (Spline|GetSplineLength (Variables|Default|GetSpline)) _progressvalue) "Local" false) false false))))

(event Collision|EventActorBeginOverlap
  (params (OtherActor :type Actor%20Object%20Reference)))

(event EventTick
  (params (DeltaSeconds :type Float%20%28single-precision%29)))

(fn ConstructionScript
  (Transformation|SetRelativeTransform (Variables|Default|GetLogoMesh) (Spline|GetTransformatSplinePoint (Variables|Default|GetSpline) 0 "Local" false) false false))