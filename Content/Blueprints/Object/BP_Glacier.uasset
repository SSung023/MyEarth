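; Pushable glacier block that the player shoves one grid step at a time, carrying any glaciers stacked above it.
; Side colliders set push direction, input and highlight; Interact box-traces the destination for blockers or seals.
; Timelines move each stacked block, then drop it by the line-traced floor distance.
; Seals ahead get moved, or turn snowy if wedged; landing on or wedging a seal destroys the glacier stack.
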(event OnComponentBeginOverlap(frontcollider)
  (params (OverlappedComponent :type Primitive%20Component%20Object%20Reference) (OtherActor :type Actor%20Object%20Reference) (OtherComp :type Primitive%20Component%20Object%20Reference) (OtherBodyIndex :type Integer) (bFromSweep :type Boolean) (SweepResult :type Hit%20Result%20Structure%20%28by%20ref%29))
  ;[1 1 1] set directionVector by activated trigger
  (Utilities|Casting|CastToPlayerCharacter OtherActor)
  (Variables|Default|SetdirectionVec "-1.000000, 0, 0")
  (Variables|Default|SetcanBePushed true)
  (Input|EnableInput (Game|GetPlayerController 0)))

(event OnComponentBeginOverlap(leftcollider)
  (params (OverlappedComponent :type Primitive%20Component%20Object%20Reference) (OtherActor :type Actor%20Object%20Reference) (OtherComp :type Primitive%20Component%20Object%20Reference) (OtherBodyIndex :type Integer) (bFromSweep :type Boolean) (SweepResult :type Hit%20Result%20Structure%20%28by%20ref%29))
  ;[1 1 1] set directionVector by activated trigger
  (Utilities|Casting|CastToPlayerCharacter OtherActor)
  (Variables|Default|SetdirectionVec "0.000000,-1.000000, 0")
  (Variables|Default|SetcanBePushed true)
  (Input|EnableInput (Game|GetPlayerController 0)))

(event OnComponentBeginOverlap(rightcollider)
  (params (OverlappedComponent :type Primitive%20Component%20Object%20Reference) (OtherActor :type Actor%20Object%20Reference) (OtherComp :type Primitive%20Component%20Object%20Reference) (OtherBodyIndex :type Integer) (bFromSweep :type Boolean) (SweepResult :type Hit%20Result%20Structure%20%28by%20ref%29))
  ;[1 1 1] set directionVector by activated trigger
  (Utilities|Casting|CastToPlayerCharacter OtherActor)
  (Variables|Default|SetdirectionVec "0.000000,1.000000, 0")
  (Variables|Default|SetcanBePushed true)
  (Input|EnableInput (Game|GetPlayerController 0)))

(event OnComponentEndOverlap(frontcollider)
  (params (OverlappedComponent :type Primitive%20Component%20Object%20Reference) (OtherActor :type Actor%20Object%20Reference) (OtherComp :type Primitive%20Component%20Object%20Reference) (OtherBodyIndex :type Integer))
  ;[1 1 1] Temp node to inactivate highlighting
  (Variables|Default|SetcanBePushed false)
  (Input|DisableInput (Game|GetPlayerController 0)))

(event OnComponentBeginOverlap(backcollider)
  (params (OverlappedComponent :type Primitive%20Component%20Object%20Reference) (OtherActor :type Actor%20Object%20Reference) (OtherComp :type Primitive%20Component%20Object%20Reference) (OtherBodyIndex :type Integer) (bFromSweep :type Boolean) (SweepResult :type Hit%20Result%20Structure%20%28by%20ref%29))
  ;[1 1 1] set directionVector by activated trigger
  (Utilities|Casting|CastToPlayerCharacter OtherActor)
  (Variables|Default|SetdirectionVec "1.000000, 0, 0")
  (Variables|Default|SetcanBePushed true)
  (Input|EnableInput (Game|GetPlayerController 0)))

(event OnComponentEndOverlap(leftcollider)
  (params (OverlappedComponent :type Primitive%20Component%20Object%20Reference) (OtherActor :type Actor%20Object%20Reference) (OtherComp :type Primitive%20Component%20Object%20Reference) (OtherBodyIndex :type Integer))
  ;[1 1 1] Temp node to inactivate highlighting
  (Variables|Default|SetcanBePushed false)
  (Input|DisableInput (Game|GetPlayerController 0)))

(event OnComponentEndOverlap(rightcollider)
  (params (OverlappedComponent :type Primitive%20Component%20Object%20Reference) (OtherActor :type Actor%20Object%20Reference) (OtherComp :type Primitive%20Component%20Object%20Reference) (OtherBodyIndex :type Integer))
  ;[1 1 1] Temp node to inactivate highlighting
  (Variables|Default|SetcanBePushed false)
  (Input|DisableInput (Game|GetPlayerController 0)))

(event OnComponentEndOverlap(backcollider)
  (params (OverlappedComponent :type Primitive%20Component%20Object%20Reference) (OtherActor :type Actor%20Object%20Reference) (OtherComp :type Primitive%20Component%20Object%20Reference) (OtherBodyIndex :type Integer))
  ;[1 1 1] Temp node to inactivate highlighting
  (Variables|Default|SetcanBePushed false)
  (Input|DisableInput (Game|GetPlayerController 0)))

(event Custom|Push
  ;[1 1 1] Check glacier condition
  (if (Variables|Default|GetcanBePushed)
    (bind _glaciers (CheckCondition|CheckUpperGlaciers))
    (Variables|Default|SetglacierList _glaciers)
    (bind _disttofloor (CheckCondition|GetDistancetoFloor))
    (bind _result (Utilities|Set|ToArray (Variables|Default|GetglacierList)))
    (for (_array_element _array_index) _result
      (Utilities|PushGlacierTypes _array_element _array_index _disttofloor (Variables|Default|GetdirectionVec)))
    (Utilities|Set|Clear (Variables|Default|GetglacierList))))

(event Custom|MoveGlacier
  (params (index :type Integer) (distToFloor :type Integer) (directionVec :type Vector))
  ;[1 1 1] Move glacier one block
  (Utilities|FlowControl|DoOnce false :!label _label
    (:Completed
      (BasicMovement|SetDirectionVec index directionVec)
      (bind _newpos (Timeline|updateGlacierPos PlayFromStart)
        (:Update
          (Transformation|SetActorLocation (+ (* (Variables|Default|GetdirectionVec) _newpos) (Variables|Default|GetcurGPos)) false false))
        (:Finished
          (Variables|Default|SetcurGPos (Transformation|GetActorLocation))
          (Variables|Default|SetcanBePushed false)
          (if (== index 0)
            (if (== distToFloor 0)
              (Utilities|WhenSealBelow
                (:out
                  (goto _label Reset)))
              (else
                _)))
          (CallFunction|FallGlacier distToFloor) ; when there's no floor
          (goto _label Reset))))))

(event Custom|FallGlacier
  (params (distToFloor :type Integer))
  ;[1 1 1] Glacier fall mechanism
  (Utilities|FlowControl|Delay 0.2)
  (bind _newheight (BasicMovement|ConvertFloorHeight distToFloor)) ; Seal 조건까지 확인
  (bind _velocity (Timeline|GlacierFalling PlayFromStart)
    (:Update
      (Transformation|SetActorLocation (+ (* _velocity (+ _newheight (Variables|Default|GetfallingDist))) (Variables|Default|GetcurGPos)) false false))
    (:Finished
      (Variables|Default|SetcurGPos (Transformation|GetActorLocation))
      (Variables|Default|SetfallingDist 0)
      (Variables|Default|SetdistToSeal 0))))

(event Custom|destroyBySeal
  (params (sealObj :type BP%20Seals%20Object%20Reference))
  ;[1 1 1] Destroy By Seal
  (bind _glaciers (CheckCondition|CheckUpperGlaciers))
  (bind _result (Utilities|Set|ToArray _glaciers))
  (for (_array_element _array_index) _result
    (if (== _array_index 0)
      (Actor|SetLifeSpan _array_element 0.3)
      (Default|SnowySeal sealObj)
      (else
        (Utilities|FlowControl|Sequence
          (:then_0
            (bind _asbp_glacier (Utilities|Casting|CastToBP_Glacier _array_element))
            (Variables|BP_Glacier_C|SetdistToSeal _asbp_glacier _array_index)
            (Variables|BP_Glacier_C|SetisSealBelow _asbp_glacier true)
            (CallFunction|FallGlacier _asbp_glacier 1)
            (Actor|SetLifeSpan _asbp_glacier 0.7))
          (:then_1
            (bind _asbp_melting_glacier (Utilities|Casting|CastToBP_MeltingGlacier _array_element))
            (Variables|/Game/Blueprints/Object/BP_MeltingGlacier.BP_MeltingGlacier_C|SetdistToSeal _asbp_melting_glacier _array_index)
            (Variables|/Game/Blueprints/Object/BP_MeltingGlacier.BP_MeltingGlacier_C|SetisSealDown _asbp_melting_glacier true)
            (Default|FallGlacier _asbp_melting_glacier 1)
            (Actor|SetLifeSpan _asbp_melting_glacier 0.7)))))))

(event EventTick
  (params (DeltaSeconds :type Float%20%28single-precision%29))
  (bind _glacier (Variables|Default|GetGlacier))
  (if (Variables|Default|GetcanBePushed)
    (Rendering|SetRenderCustomDepth _glacier true)
    (else
      (Rendering|SetRenderCustomDepth _glacier false))))

(event Input|ActionEvents|InputActionInteract
  (params (Key :type Key%20Structure :default "None"))
  ;[1 1 1] Check glacier condition
  (:Pressed
    (bind (_canmove _sealobj) (CheckCondition|IsNearSealExist))
    (if _canmove
      (Utilities|WhenSealNearby _sealobj
        (:out
          (CallFunction|Push :!label _label)))
      (else
        (bind _canmove_2 (CheckCondition|IsNearGlacierExist))
        (if (and _canmove_2 (Variables|Default|GetcanBePushed))
          (goto _label))))))

(fn ConstructionScript
  (Variables|Default|SetcurGPos (Transformation|GetActorLocation))
  (Rendering|SetRenderCustomDepth (Variables|Default|GetGlacier) false)
  (Variables|Default|SetcanBePushed false))

(fn SetDirectionVec
  (params (index :type Integer) (directionVec :type Vector))
  (if (!= index 0)
    (Variables|Default|SetdirectionVec directionVec)))

(fn FlattenVector
  (params (vec :type Vector))
  (bind (_x _y) (Math|Vector|BreakVector vec))
  (return (Math|Vector|MakeVector _x _y 0.0)))

(fn CheckUpperGlaciers
  (bind _returnvalue (Transformation|GetActorLocation))
  (bind _upperglaciers (LocalVariables|GetupperGlaciers))
  (bind _returnvalue_2 (+ _returnvalue "0, 0,150.000000"))
  (Utilities|Set|Add (LocalVariables|GetupperGlaciers) self)
  (bind _outhits (Class|KismetSystemLibrary|BoxTraceMulti _returnvalue_2 _returnvalue_2 "10.000000,10.000000,150.000000" "0, 0, 0" "TraceTypeQuery1" false 0 "ForDuration" true "(R=1.000000,G=0.000000,B=0.000000,A=1.000000)" "(R=0.000000,G=1.000000,B=0.000000,A=1.000000)" 2.0))
  (for _array_element _outhits
    (if (Actor|ActorHasTag (.HitActor (Collision|BreakHitResult _array_element)) "Glacier")
      (Utilities|Set|Add (LocalVariables|GetupperGlaciers) (.HitActor (Collision|BreakHitResult _array_element)))))
  (if (== (Utilities|Set|Length (LocalVariables|GetupperGlaciers)) 1)
    (return false _upperglaciers)
    (else
      (return true _upperglaciers))))

(fn IsNearGlacierExist
  (bind _returnvalue (Transformation|GetActorLocation))
  (bind _directionvec (Variables|Default|GetdirectionVec))
  (bind _movedistance (LocalVariables|GetmoveDistance))
  (bind _returnvalue_2 (* _directionvec _movedistance))
  (bind _returnvalue_3 (+ _returnvalue _returnvalue_2))
  (bind (_outhit _returnvalue_4) (Collision|BoxTraceByChannel _returnvalue_3 _returnvalue_3 "30.000000,30.000000,30.000000" "0, 0, 0" "TraceTypeQuery1" false 0 "None" true "(R=1.000000,G=0.000000,B=0.000000,A=1.000000)" "(R=0.000000,G=1.000000,B=0.000000,A=1.000000)" 2.0))
  (Development|PrintString (Utilities|GetDisplayName (.HitActor (Collision|BreakHitResult _outhit))))
  (return (not _returnvalue_4)))

(fn IsNearSealExist
  (bind _returnvalue (Transformation|GetActorLocation))
  (bind _directionvec (Variables|Default|GetdirectionVec))
  (bind _movedistance (LocalVariables|GetMoveDistance))
  (bind _returnvalue_2 (* _directionvec _movedistance))
  (bind _returnvalue_3 (+ _returnvalue _returnvalue_2))
  (bind _outhit (Collision|BoxTraceByChannel _returnvalue_3 _returnvalue_3 "30.000000,30.000000,30.000000" "0, 0, 0" "TraceTypeQuery1" false 0 "ForDuration" true "(R=1.000000,G=0.000000,B=0.000000,A=1.000000)" "(R=0.000000,G=0.093320,B=1.000000,A=1.000000)" 2.0))
  (bind _asbp_seals (Utilities|Casting|CastToBP_Seals (.HitActor (Collision|BreakHitResult _outhit)))
    (:then
      (return (Actor|ActorHasTag (.HitActor (Collision|BreakHitResult _outhit)) "Seal") _asbp_seals))
    (:CastFailed
      (return false 0))))

(fn GetDistancetoFloor
  (bind _returnvalue (Transformation|GetActorLocation))
  (bind _directionvec (Variables|Default|GetdirectionVec))
  (bind _movedistance (LocalVariables|GetmoveDistance))
  (bind _returnvalue_2 (* _directionvec _movedistance))
  (bind _returnvalue_3 (+ _returnvalue _returnvalue_2))
  (bind _outhit (Collision|LineTraceByChannel _returnvalue_3 (+ _returnvalue_3 "0, 0,-500.000000") "TraceTypeQuery1" false 0 "ForDuration" true "(R=1.000000,G=0.000000,B=0.000000,A=1.000000)" "(R=0.000000,G=1.000000,B=0.000000,A=1.000000)" 2.0))
  (if (Utilities|IsValid (.HitActor (Collision|BreakHitResult _outhit)))
    (if (!= (Math|Float|Truncate (/ (.Distance (Collision|BreakHitResult _outhit)) 1e+02)) 0)
      (return (Math|Float|Truncate (/ (.Distance (Collision|BreakHitResult _outhit)) 1e+02))) ; 빙하가 N칸 떨어져야 할 때
      (else
        (return 0) ; 바닥이 있는 경우
      ))
    (else
      (return -1) ; 바닥이 없는 경우
    )))

(fn CheckIsFloorExist
  (bind _returnvalue (Transformation|GetActorLocation))
  (bind _movedistance (LocalVariables|GetMoveDistance))
  (bind _directionvec (Variables|Default|GetdirectionVec))
  (bind _returnvalue_2 (* _directionvec _movedistance))
  (bind _returnvalue_3 (+ _returnvalue _returnvalue_2))
  (bind _outhit (Collision|LineTraceByChannel _returnvalue_3 (+ _returnvalue_3 "0, 0,-100.000000") "TraceTypeQuery1" false 0 "ForDuration" true "(R=1.000000,G=0.000000,B=0.000000,A=1.000000)" "(R=0.000000,G=1.000000,B=0.000000,A=1.000000)" 2.0))
  (if (Utilities|IsValid (.HitActor (Collision|BreakHitResult _outhit)))
    (Variables|Default|SetisFloorExist true)
    (else
      (Variables|Default|SetisFloorExist false))))

(fn CheckSealBelow
  (bind _returnvalue (Transformation|GetActorLocation))
  (bind _outhit (Collision|LineTraceByChannel _returnvalue (+ _returnvalue "0, 0,-100.000000") "TraceTypeQuery1" false 0 "ForDuration" true "(R=1.000000,G=0.000000,B=0.000000,A=1.000000)" "(R=0.000000,G=1.000000,B=0.000000,A=1.000000)" 2.0))
  (if (Actor|ActorHasTag (.HitActor (Collision|BreakHitResult _outhit)) "Seal")
    (bind _asbp_seals (Utilities|Casting|CastToBP_Seals (.HitActor (Collision|BreakHitResult _outhit)))
      (:then
        (return true _asbp_seals))
      (:CastFailed
        _)))
  (return false 0))

(fn ConvertFloorHeight
  (params (distToFloor :type Integer))
  (if (== distToFloor -1)
    (return 1)
    (elif (Variables|Default|GetisSealBelow)
      (return (Variables|Default|GetdistToSeal))
      (else
        (return distToFloor)))))