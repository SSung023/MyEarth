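; Construction-time brush actor, named as a dummy glacier dirt brush, that fills a box with a 3D grid of child actors.
; Unless Designing is set, the construction script snaps the actor's X and Y to a 50-unit grid via MakeLocationSnap.
; It then derives per-axis counts from Endpoint and BlockSize and adds child actor components in nested loops, raised half a block in Z.
; It has no runtime logic.
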(event EventBeginPlay)

(event Collision|EventActorBeginOverlap
  (params (OtherActor :type Actor%20Object%20Reference)))

(event EventTick
  (params (DeltaSeconds :type Float%20%28single-precision%29)))

(fn ConstructionScript
  (bind _returnvalue (Transformation|GetActorLocation))
  (bind _endpoint (Variables|Option|GetEndpoint))
  (bind _blocksize (Variables|Option|GetBlockSize))
  (if (not (Variables|Option|GetDesigning))
    (Variables|Construction|SetHalfBlockSize (Math|Conversions|ToFloat(Integer) (/ (Variables|Option|GetBlockSize) 2)))
    (bind _result (CallFunction|MakeLocationSnap (.x _returnvalue)))
    (bind _result_2 (CallFunction|MakeLocationSnap (.y _returnvalue)))
    (Transformation|SetActorLocation (Math|Vector|MakeVector _result _result_2 (.z _returnvalue)) false false)
    (Variables|Construction|SetXCount (/ (Math|Float|Round (.x _endpoint)) _blocksize))
    (Variables|Construction|SetYCount (/ (Math|Float|Round (.y _endpoint)) _blocksize))
    (Variables|Construction|SetZCount (/ (Math|Float|Round (+ (.z _endpoint) (Variables|Construction|GetHalfBlockSize))) _blocksize))
    (for _index (range 0 (Variables|Construction|GetXCount))
      (for _index_2 (range 0 (Variables|Construction|GetYCount))
        (for _index_3 (range 0 (Variables|Construction|GetZCount))
          (AddComponent|AddChildActorComponent false (Math|Transform|MakeTransform (Math|Vector|MakeVector (Math|Conversions|ToFloat(Integer) (* _index (Variables|Option|GetBlockSize))) (Math|Conversions|ToFloat(Integer) (* _index_2 (Variables|Option|GetBlockSize))) (+ (Math|Conversions|ToFloat(Integer) (* _index_3 (Variables|Option|GetBlockSize))) (Variables|Construction|GetHalfBlockSize))))))))))

(fn MakeLocationSnap
  (params (Axis :type Float%20%28single-precision%29))
  (bind _returnvalue (Math|Float|%(Float) Axis 5e+01))
  (if (== _returnvalue 0.0)
    (LocalVariables|SetSnappedAxis Axis)
    (else
      (LocalVariables|SetRemains _returnvalue)
      (if (> (Math|Float|Absolute(Float) (LocalVariables|GetRemains)) 25.0)
        (LocalVariables|SetCompensator (- 5e+01 (LocalVariables|GetRemains)))
        (else
          (LocalVariables|SetCompensator (* (LocalVariables|GetRemains) -1.0))))
      (LocalVariables|SetSnappedAxis (+ Axis (LocalVariables|GetCompensator)))))
  (return (LocalVariables|GetSnappedAxis)))