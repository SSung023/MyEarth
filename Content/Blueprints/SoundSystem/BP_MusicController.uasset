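; BP_MusicController is a music control Blueprint that starts a configured background track with a fade-in on BeginPlay.
; It forwards play, stop, change and toggle events, plus an is-playing query, to the BP_Inst_MyEarth game instance, which handles BGM playback.
; A key binding marked as a temporary solution flip-flops music off and on.
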(event Custom|Play%20BGM
  (params (BGM%20to%20Play :type Sound%20Cue%20Object%20Reference) (FadeIn :type Float%20%28single-precision%29))
  ;[0.7894 1 0.1357] Music Control
  (Class|IMusicManager|PlayBGM(Message) (Variables|Default|GetGameInstance) BGM%20to%20Play FadeIn))

(event Custom|Stop%20BGM
  (params (FadeOut :type Float%20%28single-precision%29))
  ;[0.7894 1 0.1357] Music Control
  (Class|IMusicManager|StopBGM(Message) (Variables|Default|GetGameInstance) FadeOut))

(event Custom|Change%20BGM
  (params (BGM%20to%20Play :type Sound%20Cue%20Object%20Reference) (FadeOut :type Float%20%28single-precision%29) (FadeIn :type Float%20%28single-precision%29))
  ;[0.7894 1 0.1357] Music Control
  (Class|IMusicManager|ChangeBGM(Message) (Variables|Default|GetGameInstance) BGM%20to%20Play FadeOut FadeIn))

(event Custom|ToggleMusic
  (params (SetMusicPlay :type Boolean))
  ;[0.7894 1 0.1357] Music Control
  (Default|ToggleMusic (Variables|Default|GetGameInstance) SetMusicPlay))

(event EventBeginPlay
  (Variables|Default|SetGameInstance (CallFunction|GetMyearthGameInstance))
  (bind _music_to_play (Variables|Option|GetMusic%20to%20Play)
    (:then
      (Class|IMusicManager|PlayBGM(Message) (Variables|Default|GetGameInstance) _music_to_play (Variables|Option|GetFade%20In%20Duration)))
    (:else)))

(event Input|KeyboardEvents|Shift1
  (params (Key :type Key%20Structure :default "None"))
  ;[1 0.2207 0.3305] Temporary Solution
  (:Pressed
    (Utilities|FlowControl|FlipFlop
      (:A
        (CallFunction|ToggleMusic false))
      (:B
        (CallFunction|ToggleMusic true)))))

(fn ConstructionScript)

(fn GetMyearthGameInstance
  (bind _asbp_inst_my_earth (Utilities|Casting|CastToBP_Inst_MyEarth (Game|GetGameInstance)))
  (return _asbp_inst_my_earth))

(fn IsPlaying
  (return (Default|IsPlayingBGM (Variables|Default|GetGameInstance))))