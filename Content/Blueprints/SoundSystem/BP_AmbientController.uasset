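; BP_AmbientController is a controller that starts and manages ambient sound through the BP_Inst_MyEarth game instance.
; On BeginPlay it caches that instance and, if an ambient sound is set, asks it to play that sound with a fade-in.
; Its play, stop, change, toggle and playing-state calls forward to the game instance.
; A key binding marked as temporary flip-flops the ambient off and on.
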(event Custom|Play%20AMB
  (params (AMB%20to%20Play :type Sound%20Cue%20Object%20Reference) (FadeIn :type Float%20%28single-precision%29))
  ;[0.7894 1 0.1357] Music Control
  (Default|PlayAMB (Variables|Default|GetGameInstance) AMB%20to%20Play FadeIn))

(event Custom|Stop%20AMB
  (params (FadeOut :type Float%20%28single-precision%29))
  ;[0.7894 1 0.1357] Music Control
  (Default|StopAMB (Variables|Default|GetGameInstance) FadeOut))

(event Custom|Change%20AMB
  (params (AMB%20to%20Play :type Sound%20Cue%20Object%20Reference) (FadeOut :type Float%20%28single-precision%29) (FadeIn :type Float%20%28single-precision%29))
  ;[0.7894 1 0.1357] Music Control
  (Default|ChangeAMB (Variables|Default|GetGameInstance) AMB%20to%20Play FadeOut FadeIn))

(event Custom|ToggleAmbient
  (params (SetAmbientPlay :type Boolean))
  ;[0.7894 1 0.1357] Music Control
  (Default|ToggleAmbient (Variables|Default|GetGameInstance) SetAmbientPlay))

(event EventBeginPlay
  (Variables|Default|SetGameInstance (CallFunction|GetMyearthGameInstance))
  (bind _ambient_to_play (Variables|Option|GetAmbient%20to%20Play)
    (:then
      (Class|IAmbientManager|PlayAMB(Message) (Variables|Default|GetGameInstance) _ambient_to_play (Variables|Option|GetFade%20In%20Duration)))
    (:else)))

(event Input|KeyboardEvents|Shift2
  (params (Key :type Key%20Structure :default "None"))
  ;[1 0.2207 0.3305] Temporary Solution
  (:Pressed
    (Utilities|FlowControl|FlipFlop
      (:A
        (CallFunction|ToggleAmbient false))
      (:B
        (CallFunction|ToggleAmbient true)))))

(fn ConstructionScript)

(fn GetMyearthGameInstance
  (bind _asbp_inst_my_earth (Utilities|Casting|CastToBP_Inst_MyEarth (Game|GetGameInstance)))
  (return _asbp_inst_my_earth))

(fn IsPlayingAMB
  (return (Default|IsPlayingAMB (Variables|Default|GetGameInstance))))