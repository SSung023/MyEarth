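; EasyFog actor that renders a configurable fog card for placing fog in a level.
; The construction script creates a dynamic material instance on FogCard, using PathtracerToggle to pick the path tracer or standard source material.
; Both branches push the same exposed tint, density, fading, texture map, emissive and wind settings into that material, then set shadow casting.
; The event graph has no active logic, so this Blueprint does no runtime updates.
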(event EventBeginPlay)

(event Collision|EventActorBeginOverlap
  (params (OtherActor :type Actor%20Object%20Reference)))

(event EventTick
  (params (DeltaSeconds :type Float%20%28single-precision%29)))

(fn ConstructionScript
  (bind _fogcard (Variables|EasyfogSettings|GetFogCard))
  (if (Variables|EasyfogSettings|GetPathtracer%20Toggle)
    (bind _returnvalue (Rendering|Material|CreateDynamicMaterialInstance _fogcard 0 (Variables|EasyfogSettings|GetPathtracer%20Material) "None" :!class /Script/Engine.PrimitiveComponent))
    (bind _output_get (Variables|EasyfogSettings|SetFog%20Material%20Instance _returnvalue))
    (Rendering|Material|SetVectorParameterValue _output_get "Base Color Tint" (Variables|EasyfogSettings|GetBase%20Color%20Tint) :!class /Script/Engine.MaterialInstanceDynamic)
    (Rendering|Material|SetScalarParameterValue (Variables|EasyfogSettings|GetFog%20Material%20Instance) "Base Color Contrast" (Variables|EasyfogSettings|GetBase%20Color%20Contrast) :!class /Script/Engine.MaterialInstanceDynamic)
    (Rendering|Material|SetScalarParameterValue (Variables|EasyfogSettings|GetFog%20Material%20Instance) "Base Color Intensity" (Variables|EasyfogSettings|GetBase%20Color%20Intensity) :!class /Script/Engine.MaterialInstanceDynamic)
    (Rendering|Material|SetScalarParameterValue (Variables|EasyfogSettings|GetFog%20Material%20Instance) "Fading Distance" (Variables|EasyfogSettings|GetGeometry%20Fading%20Distance) :!class /Script/Engine.MaterialInstanceDynamic)
    (Rendering|Material|SetScalarParameterValue (Variables|EasyfogSettings|GetFog%20Material%20Instance) "Fog Density" (Variables|EasyfogSettings|GetFog%20Density) :!class /Script/Engine.MaterialInstanceDynamic)
    (Rendering|Material|SetScalarParameterValue (Variables|EasyfogSettings|GetFog%20Material%20Instance) "Camera Fading Distance" (Variables|EasyfogSettings|GetCamera%20Fading%20Distance) :!class /Script/Engine.MaterialInstanceDynamic)
    (Rendering|Material|SetScalarParameterValue (Variables|EasyfogSettings|GetFog%20Material%20Instance) "Normal Intensity" (Variables|EasyfogSettings|GetNormal%20Map%20Intensity) :!class /Script/Engine.MaterialInstanceDynamic)
    (Rendering|Material|SetTextureParameterValue (Variables|EasyfogSettings|GetFog%20Material%20Instance) "Opacity Map" (Variables|EasyfogSettings|GetOpacity%20Map))
    (Rendering|Material|SetTextureParameterValue (Variables|EasyfogSettings|GetFog%20Material%20Instance) "Base Color Map" (Variables|EasyfogSettings|GetBase%20Color%20Map))
    (Rendering|Material|SetTextureParameterValue (Variables|EasyfogSettings|GetFog%20Material%20Instance) "FogNormals" (Variables|EasyfogSettings|GetNormal%20Map))
    (Rendering|Material|SetScalarParameterValue (Variables|EasyfogSettings|GetFog%20Material%20Instance) "Emissive Intensity" (Variables|EasyfogSettings|GetEmissive%20Intensity) :!class /Script/Engine.MaterialInstanceDynamic)
    (Rendering|Material|SetScalarParameterValue (Variables|EasyfogSettings|GetFog%20Material%20Instance) "Wind?" (Variables|WindControls|GetWind%20:%20Yes/No) :!class /Script/Engine.MaterialInstanceDynamic)
    (Rendering|Material|SetScalarParameterValue (Variables|EasyfogSettings|GetFog%20Material%20Instance) "Wind Speed Y" (Variables|WindControls|GetWind%20Speed%20Y) :!class /Script/Engine.MaterialInstanceDynamic)
    (Rendering|Material|SetScalarParameterValue (Variables|EasyfogSettings|GetFog%20Material%20Instance) "Wind Speed X" (Variables|WindControls|GetWind%20Speed%20X) :!class /Script/Engine.MaterialInstanceDynamic)
    (Rendering|Material|SetScalarParameterValue (Variables|EasyfogSettings|GetFog%20Material%20Instance) "Wind Noise Tiling" (Variables|WindControls|GetWind%20Noise%20Tiling) :!class /Script/Engine.MaterialInstanceDynamic)
    (Rendering|Material|SetScalarParameterValue (Variables|EasyfogSettings|GetFog%20Material%20Instance) "Wind Noise Contrast" (Variables|WindControls|GetWind%20Noise%20Contrast) :!class /Script/Engine.MaterialInstanceDynamic)
    (Rendering|Material|SetScalarParameterValue (Variables|EasyfogSettings|GetFog%20Material%20Instance) "View Angle Fade" (Variables|EasyfogSettings|GetView%20Angle%20Fade) :!class /Script/Engine.MaterialInstanceDynamic)
    (Rendering|SetCastShadow (Variables|EasyfogSettings|GetFogCard) (Variables|EasyfogSettings|GetCast%20Shadow?))
    (else
      (bind _returnvalue_2 (Rendering|Material|CreateDynamicMaterialInstance _fogcard 0 (LocalVariables|GetSource%20Material) "None" :!class /Script/Engine.PrimitiveComponent))
      (bind _output_get_2 (Variables|EasyfogSettings|SetFog%20Material%20Instance _returnvalue_2))
      (Rendering|Material|SetVectorParameterValue _output_get_2 "Base Color Tint" (Variables|EasyfogSettings|GetBase%20Color%20Tint) :!class /Script/Engine.MaterialInstanceDynamic)
      (Rendering|Material|SetScalarParameterValue (Variables|EasyfogSettings|GetFog%20Material%20Instance) "Base Color Contrast" (Variables|EasyfogSettings|GetBase%20Color%20Contrast) :!class /Script/Engine.MaterialInstanceDynamic)
      (Rendering|Material|SetScalarParameterValue (Variables|EasyfogSettings|GetFog%20Material%20Instance) "Base Color Intensity" (Variables|EasyfogSettings|GetBase%20Color%20Intensity) :!class /Script/Engine.MaterialInstanceDynamic)
      (Rendering|Material|SetScalarParameterValue (Variables|EasyfogSettings|GetFog%20Material%20Instance) "Fading Distance" (Variables|EasyfogSettings|GetGeometry%20Fading%20Distance) :!class /Script/Engine.MaterialInstanceDynamic)
      (Rendering|Material|SetScalarParameterValue (Variables|EasyfogSettings|GetFog%20Material%20Instance) "Fog Density" (Variables|EasyfogSettings|GetFog%20Density) :!class /Script/Engine.MaterialInstanceDynamic)
      (Rendering|Material|SetScalarParameterValue (Variables|EasyfogSettings|GetFog%20Material%20Instance) "Camera Fading Distance" (Variables|EasyfogSettings|GetCamera%20Fading%20Distance) :!class /Script/Engine.MaterialInstanceDynamic)
      (Rendering|Material|SetScalarParameterValue (Variables|EasyfogSettings|GetFog%20Material%20Instance) "Normal Intensity" (Variables|EasyfogSettings|GetNormal%20Map%20Intensity) :!class /Script/Engine.MaterialInstanceDynamic)
      (Rendering|Material|SetTextureParameterValue (Variables|EasyfogSettings|GetFog%20Material%20Instance) "Opacity Map" (Variables|EasyfogSettings|GetOpacity%20Map))
      (Rendering|Material|SetTextureParameterValue (Variables|EasyfogSettings|GetFog%20Material%20Instance) "Base Color Map" (Variables|EasyfogSettings|GetBase%20Color%20Map))
      (Rendering|Material|SetTextureParameterValue (Variables|EasyfogSettings|GetFog%20Material%20Instance) "FogNormals" (Variables|EasyfogSettings|GetNormal%20Map))
      (Rendering|Material|SetScalarParameterValue (Variables|EasyfogSettings|GetFog%20Material%20Instance) "Emissive Intensity" (Variables|EasyfogSettings|GetEmissive%20Intensity) :!class /Script/Engine.MaterialInstanceDynamic)
      (Rendering|Material|SetScalarParameterValue (Variables|EasyfogSettings|GetFog%20Material%20Instance) "Wind?" (Variables|WindControls|GetWind%20:%20Yes/No) :!class /Script/Engine.MaterialInstanceDynamic)
      (Rendering|Material|SetScalarParameterValue (Variables|EasyfogSettings|GetFog%20Material%20Instance) "Wind Speed Y" (Variables|WindControls|GetWind%20Speed%20Y) :!class /Script/Engine.MaterialInstanceDynamic)
      (Rendering|Material|SetScalarParameterValue (Variables|EasyfogSettings|GetFog%20Material%20Instance) "Wind Speed X" (Variables|WindControls|GetWind%20Speed%20X) :!class /Script/Engine.MaterialInstanceDynamic)
      (Rendering|Material|SetScalarParameterValue (Variables|EasyfogSettings|GetFog%20Material%20Instance) "Wind Noise Tiling" (Variables|WindControls|GetWind%20Noise%20Tiling) :!class /Script/Engine.MaterialInstanceDynamic)
      (Rendering|Material|SetScalarParameterValue (Variables|EasyfogSettings|GetFog%20Material%20Instance) "Wind Noise Contrast" (Variables|WindControls|GetWind%20Noise%20Contrast) :!class /Script/Engine.MaterialInstanceDynamic)
      (Rendering|Material|SetScalarParameterValue (Variables|EasyfogSettings|GetFog%20Material%20Instance) "View Angle Fade" (Variables|EasyfogSettings|GetView%20Angle%20Fade) :!class /Script/Engine.MaterialInstanceDynamic)
      (Rendering|SetCastShadow (Variables|EasyfogSettings|GetFogCard) (Variables|EasyfogSettings|GetCast%20Shadow?)))))